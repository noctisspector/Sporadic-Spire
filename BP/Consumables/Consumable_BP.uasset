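; Consumable actor that calls in an airstrike around its own location when play begins.
; It reads the hard-coded "Airstrike" row of the consumable data table, then uses a delayed loop with randomized timing to spawn the configured number of projectiles.
; Each spawns at a random horizontal offset and set height, pointing straight down, and receives its speed, damage, knockback, radius, stun and explosion effects from that row.
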(event EventBeginPlay
  (|CallParentFunction)
  ;[1 1 1] Get Data Table Properties
  (bind __ (CallFunction|GetDataTableProperties))
  (Variables|Default|SetProperties __)
  (Utilities|ForLoopwithDelay 1 (.firecount (Variables|Default|GetProperties)) (Math|Random|RandomFloatinRange (.X (Math|Vector2D|BreakVector2D (.firerandomness (Variables|Default|GetProperties)))) (.Y (Math|Vector2D|BreakVector2D (.firerandomness (Variables|Default|GetProperties)))))
    (:Loop%20Body
      (bind _returnvalue (Game|SpawnActorfromClass (.projectileclass (Variables|Default|GetProperties)) (Math|Transform|MakeTransform (+ (Transformation|GetActorLocation) (Math|Vector|MakeVector (Math|Random|RandomFloatinRange (Utilities|Invert(float) (.X (Math|Vector2D|BreakVector2D (.firerandom (Variables|Default|GetProperties))))) (.X (Math|Vector2D|BreakVector2D (.firerandom (Variables|Default|GetProperties))))) (Math|Random|RandomFloatinRange (Utilities|Invert(float) (.Y (Math|Vector2D|BreakVector2D (.firerandom (Variables|Default|GetProperties))))) (.Y (Math|Vector2D|BreakVector2D (.firerandom (Variables|Default|GetProperties))))) (.fireheight (Variables|Default|GetProperties)))) (Math|Rotator|MakeRotator 0.0 -9e+01 0.0) "1,1,1") "Undefined" 0 0))
      (Default|SetDefaultValues _returnvalue (.projectilespeed (Variables|Default|GetProperties)) (.explosioneffect (Variables|Default|GetProperties)) (.damage (Variables|Default|GetProperties)) (.knockback (Variables|Default|GetProperties)) (.damageradius (Variables|Default|GetProperties)) 0 (.stuntime (Variables|Default|GetProperties)) 0.0 0 0 (.expsound (Variables|Default|GetProperties))))))

(fn ConstructionScript)

(fn GetDataTableProperties
  (bind _returnvalue (Utilities|GetDataTableRow "/Game/BP/Consumables/ConsumableTable.ConsumableTable" "Airstrike")
    (:then
      (return _returnvalue))))