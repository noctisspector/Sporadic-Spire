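; Enemy spawn tile that runs the wave loop, from countdown (held for a trigger in tutorials) to win menu.
; Each wave builds a class list by weight and minimum wave, then spawns it in random order near SpawnPoint with per-class delays.
; Tick polls for all enemies dead, then awards gold, harvests lumber huts, saves Wave Points and schedules the next wave.
; Spawn count grows linearly, health exponentially by difficulty.
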(event Custom|Start%20Waves%20Tutorial
  (bind __ (Utilities|GameInstance))
  (bind _initial_delay (Variables|SpawnSettings|GetInitial%20Delay))
  (bind _btutorial (Variables|/Game/BP/Global_GI.Global_GI_C|GetbTutorial __))
  (bind _returnvalue (select _btutorial 5.0 _initial_delay))
  ;[1 1 1] Init
  (CallFunction|UpdateGamemodeWave)
  (CallFunction|MakeCountdown (Math|Float|Truncate _returnvalue))
  (Utilities|FlowControl|Delay _returnvalue)
  (Variables|Default|SetbSpawnBoolean true))

(event Custom|Make%20Countdown
  (params (Amount :type Integer))
  ;[1 1 1] Make Countdown
  (bind _returnvalue (UserInterface|CreateWidget "/Game/BP/Widget/Countdown_Widget.Countdown_Widget_C" (Game|GetPlayerController 0)))
  (Default|Initialize _returnvalue Amount)
  (UserInterface|Viewport|AddtoViewport _returnvalue 0))

(event EventBeginPlay
  (bind __ (Utilities|GameInstance))
  (bind _initial_delay (Variables|SpawnSettings|GetInitial%20Delay))
  (bind _btutorial (Variables|/Game/BP/Global_GI.Global_GI_C|GetbTutorial __))
  (bind _returnvalue (select _btutorial 5.0 _initial_delay))
  ;[1 1 1] Init
  (|CallParentFunction)
  (Variables|/Game/BP/Player_BP.Player_BP_C|SetEnemy%20Spawn (Utilities|Player) self)
  (Variables|/Game/BP/Global_GI.Global_GI_C|Setspawn (Utilities|GameInstance) self)
  (if (not _btutorial)
    (CallFunction|UpdateGamemodeWave)
    (CallFunction|MakeCountdown (Math|Float|Truncate _returnvalue))
    (Utilities|FlowControl|Delay _returnvalue)
    (Variables|Default|SetbSpawnBoolean true)))

(event EventTick
  (params (DeltaSeconds :type Float%20%28single-precision%29))
  (bind _spawn_point (Variables|Default|GetSpawn%20Point))
  (bind _between_delay (Variables|SpawnSettings|GetBetween%20Delay))
  (bind _enemy_spawn_list (Variables|Default|GetEnemy%20Spawn%20List))
  (bind _wave_wp_reward (Variables|Default|GetWave%20WP%20Reward))
  (bind _win_wp_reward (Variables|Default|GetWin%20WP%20Reward))
  (bind _returnvalue (Utilities|Array|Length _enemy_spawn_list))
  (bind _returnvalue_2 (Transformation|GetWorldLocation _spawn_point))
  (bind _randomlocation (Class|NavigationSystemV1|GetRandomPointinNavigableRadius _returnvalue_2 1e+02 0 0))
  (|CallParentFunction DeltaSeconds)
  (Utilities|FlowControl|Sequence
    (:then_0
      (if (Variables|Default|GetbSpawnBoolean)
        (Utilities|FlowControl|Sequence
          (:then_0
            (Utilities|FlowControl|DoOnce false
              (:Completed
                (Variables|Default|SetbInitialSpawnBoolean true))))
          (:then_1
            (Variables|Default|SetbSpawnBoolean false)
            ;[1 1 1] Enemy Spawn
            (for _array_element (Variables|SpawnSettings|GetSpawn%20Data)
              ;;[1 1 1] Min Wave
              (if (>= (Variables|Default|GetCurrent%20Wave) (.minwave _array_element))
                (for _index (range 1 (Math|Float|Round (* (Variables|SpawnSettings|GetBase%20Spawn%20Count) (.weight _array_element))))
                  (Utilities|Array|Add (Variables|Default|GetEnemy%20Spawn%20List) (.class _array_element)))))
            ;[1 1 1] Spawn Same-Class Entities
            (bind _output_get (Variables|Default|SetEnemy%20Spawn%20List%20Length _returnvalue))
            (Utilities|ForLoopwithDelay 0 (- _output_get 1) (Variables|Default|GetEnemy%20Spawn%20Delay)
              (:Loop%20Body
                (Variables|Default|SetEnemy%20Spawn%20List%20Random%20Index (Math|Random|RandomIntegerinRange 0 (- _returnvalue 1)))
                (Variables|Default|SetEnemy%20Spawn%20Delay (.Spawn%20Delay (Utilities|GetClassDefaults (Utilities|Array|Get(acopy) _enemy_spawn_list (Variables|Default|GetEnemy%20Spawn%20List%20Random%20Index)))))
                (bind _returnvalue_3 (Game|SpawnActorfromClass (Utilities|Array|Get(acopy) _enemy_spawn_list (Variables|Default|GetEnemy%20Spawn%20List%20Random%20Index)) (Math|Transform|MakeTransform (Math|Vector|MakeVector (.x _randomlocation) (.y _randomlocation) (.Z (Math|Vector|BreakVector _returnvalue_2))) "0, 0, 0" "1,1,1") "AdjustIfPossibleButAlwaysSpawn" 0 0))
                (Default|SetHealthModifier _returnvalue_3 (Variables|Default|GetCurrent%20Health%20Modifier))
                (Utilities|Array|Add (Variables|Default|GetWave%20Enemies) _returnvalue_3)
                (Utilities|Array|RemoveIndex (Variables|Default|GetEnemy%20Spawn%20List) (Variables|Default|GetEnemy%20Spawn%20List%20Random%20Index))))))))
    (:then_1
      ;[1 1 1] Determine if all Enemies are Dead
      (if (Variables|Default|GetbInitialSpawnBoolean)
        (Variables|Default|SetbAliveEnemy false)
        (for _array_element_2 (Variables|Default|GetWave%20Enemies)
          (if (not (Variables|Default|GetbAliveEnemy))
            (if (not (Variables|/Game/BP/Enemy/Enemy_BP.Enemy_BP_C|GetbDead _array_element_2))
              (Variables|Default|SetbAliveEnemy true))))
        ;[1 1 1] New Wave
        (if (Math|Boolean|ANDBoolean (not (Variables|Default|GetbAliveEnemy)) (not (Variables|Default|GetbNewWave)) (<= (Utilities|Array|Length (Variables|Default|GetEnemy%20Spawn%20List)) 0))
          (Variables|Default|SetbNewWave true)
          (bind _total_gold (CallFunction|HarvestLumberHuts))
          (CallFunction|NewWaveWidget _total_gold _wave_wp_reward)
          (CallFunction|RewardWP _wave_wp_reward)
          (CallFunction|MakeCountdown (Math|Float|Truncate _between_delay))
          (Default|TutorialKilledWave (Utilities|Player))
          (Utilities|FlowControl|Delay _between_delay)
          (Math|Integer|IncrementInt (Variables|Default|GetCurrent%20Wave)
            (:%20%20
              (CallFunction|UpdateGamemodeWave)
              (Variables|SpawnSettings|SetBase%20Spawn%20Count (+ (Variables|SpawnSettings|GetBase%20Spawn%20Count) (Variables|SpawnSettings|GetBase%20Spawn%20Count%20Increment)))
              (for _array_element_3 (Variables|Default|GetWave%20Enemies)
                (Default|Destroy _array_element_3))
              (Variables|Default|SetbSpawnBoolean true)
              (Utilities|Array|Clear (Variables|Default|GetWave%20Enemies))
              (bind _y (CallFunction|EnemyProgressionFunction (Math|Conversions|ToFloat(Integer) (Variables|Default|GetCurrent%20Wave))))
              (Variables|Default|SetCurrent%20Health%20Modifier _y)
              (Variables|Default|SetbNewWave false)
              ;[1 1 1] Winning
              (if (>= (Variables|Default|GetCurrent%20Wave) (Variables|SpawnSettings|GetWin%20Wave))
                (Utilities|FlowControl|DoOnce false
                  (:Completed
                    (Game|SetGamePaused true)
                    (bind _returnvalue_4 (UserInterface|CreateWidget "/Game/BP/Widget/WinMenu_BP.WinMenu_BP_C" (Game|GetPlayerController 0)))
                    (UserInterface|Viewport|AddtoViewport _returnvalue_4 0)
                    (Variables|/Game/BP/Widget/WinMenu_BP.WinMenu_BP_C|SetWP _returnvalue_4 _win_wp_reward)
                    (CallFunction|RewardWP _win_wp_reward)))))))))))

(fn ConstructionScript
  (|CallParentFunction))

(fn UpdateGamemodeWave
  (Variables|/Game/BP/MainGamemode_BP.MainGamemode_BP_C|SetCurrent%20Wave (Utilities|Gamemode) (Variables|Default|GetCurrent%20Wave)))

(fn HarvestLumberHuts
  (bind _wave_base_gold (Variables|SpawnSettings|GetWave%20Base%20Gold))
  (bind _outactors (Actor|GetAllActorsOfClass "/Game/BP/Tiles/PlayerTiles/LumberHut_BP.LumberHut_BP_C"))
  (for _array_element _outactors
    (bind _harvested_gold (Default|Harvest _array_element))
    (LocalVariables|SetHarvested%20Gold (+ _harvested_gold (LocalVariables|GetHarvested%20Gold))))
  (Default|GainGold (Utilities|Player) _wave_base_gold)
  (return (+ (LocalVariables|GetHarvested%20Gold) _wave_base_gold)))

(fn NewWaveWidget
  (params (Gold :type Integer) (WP :type Integer))
  (bind _returnvalue (UserInterface|CreateWidget "/Game/BP/Widget/WaveEnd_BP.WaveEnd_BP_C" (Game|GetPlayerController 0)))
  (UserInterface|Viewport|AddtoViewport _returnvalue 0)
  (Default|PlayAnimation _returnvalue (Variables|Default|GetCurrent%20Wave) Gold WP))

(fn RewardWP
  (params (Amount :type Integer))
  (bind __ (Utilities|GameInstance))
  (bind _globalsave (Variables|/Game/BP/Global_GI.Global_GI_C|GetGlobalSave __))
  (bind _output_get (Variables|/Game/BP/Saves/Global_SaveGame.Global_SaveGame_C|SetWave%20Points _globalsave (+ Amount (Variables|/Game/BP/Saves/Global_SaveGame.Global_SaveGame_C|GetWave%20Points _globalsave))))
  (Variables|/Game/BP/Global_GI.Global_GI_C|SetWp __ _output_get)
  (SaveGame|SaveGametoSlot _globalsave "Global"))

(fn EnemyProgressionFunction
  (params (X :type Float%20%28single-precision%29))
  (bind _enemy_progression_base (Variables|SpawnSettings|GetEnemy%20Progression%20Base))
  (bind _enemy_progression_scale (Variables|SpawnSettings|GetEnemy%20Progression%20Scale))
  (return (+ (* (- (Math|Float|Power (Utilities|Select :Index (Variables|/Game/BP/Global_GI.Global_GI_C|GetDifficulty (Utilities|GameInstance)) :NewEnumerator0 (.easy _enemy_progression_base) :NewEnumerator1 (.medium _enemy_progression_base) :NewEnumerator2 (.hard _enemy_progression_base)) X) 1.0) (Utilities|Select :Index (Variables|/Game/BP/Global_GI.Global_GI_C|GetDifficulty (Utilities|GameInstance)) :NewEnumerator0 (.easy _enemy_progression_scale) :NewEnumerator1 (.medium _enemy_progression_scale) :NewEnumerator2 (.hard _enemy_progression_scale))) 1.0)))