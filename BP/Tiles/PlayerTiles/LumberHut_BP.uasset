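; Lumber hut player tile that earns the player gold from tree tiles within its function radius.
; Harvest scans every Tile_BP actor, adds a gold increase for each nearby one flagged as Tree, then pays the total to the player and returns it.
; GoldPerRound repeats the same scan to report the income without paying it.
; Event graph and construction script only call the parent.
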(event EventBeginPlay
  (|CallParentFunction))

(event Collision|EventActorBeginOverlap
  (params (OtherActor :type Actor%20Object%20Reference))
  (|CallParentFunction OtherActor) ; This node is disabled and will not be called.\nDrag off pins to build functionality.
)

(event EventTick
  (params (DeltaSeconds :type Float%20%28single-precision%29))
  (|CallParentFunction DeltaSeconds) ; This node is disabled and will not be called.\nDrag off pins to build functionality.
)

(fn ConstructionScript
  (|CallParentFunction))

(fn Harvest
  (bind _outactors (Actor|GetAllActorsOfClass "/Game/BP/Tile_BP.Tile_BP_C"))
  (for _array_element _outactors
    (bind _btree (CallFunction|GetHarvestable _array_element))
    (if _btree
      (if (< (Transformation|GetDistanceTo _array_element) (Variables|Default|GetFunction%20Radius))
        (LocalVariables|SetGold%20Gain (+ (LocalVariables|GetGold%20Gain) (Variables|Default|GetGold%20Increase))))))
  (Default|GainGold (Utilities|Player) (LocalVariables|GetGold%20Gain))
  (return (LocalVariables|GetGold%20Gain)))

(fn GetHarvestable
  (params (self2 :type Tile%20BP%20Object%20Reference))
  (return (Variables|/Game/BP/Tile_BP.Tile_BP_C|GetbTree self2)))

(fn GoldPerRound
  (bind _outactors (Actor|GetAllActorsOfClass "/Game/BP/Tile_BP.Tile_BP_C"))
  (for _array_element _outactors
    (bind _btree (CallFunction|GetHarvestable _array_element))
    (if _btree
      (if (< (Transformation|GetDistanceTo _array_element) (Variables|Default|GetFunction%20Radius))
        (LocalVariables|SetGold%20Gain (+ (LocalVariables|GetGold%20Gain) (Variables|Default|GetGold%20Increase))))))
  (return (LocalVariables|GetGold%20Gain)))