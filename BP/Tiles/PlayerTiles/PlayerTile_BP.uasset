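; Player tile Blueprint that carries a function radius and keeps track of the tile class set as its previous tile.
; On BeginPlay the radius sizes both a sphere mesh and a collision sphere, and the gradient enable/disable events show or hide that mesh.
; If the previous tile is a dock, it hides the ground mesh and spawns that class as a child actor with box collision disabled.
; Upgrade is an empty stub.
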(event EventBeginPlay
  (|CallParentFunction)
  (CallFunction|SetFunctionRadius (Variables|Properties|GetFunction%20Radius)))

(event Collision|EventActorBeginOverlap
  (params (OtherActor :type Actor%20Object%20Reference))
  (|CallParentFunction OtherActor) ; This node is disabled and will not be called.\nDrag off pins to build functionality.
)

(event EventTick
  (params (DeltaSeconds :type Float%20%28single-precision%29))
  (|CallParentFunction DeltaSeconds) ; This node is disabled and will not be called.\nDrag off pins to build functionality.
)

(event EventEnableGradient
  (params (Material :type Material%20Interface%20Object%20Reference))
  (|CallParentFunction Material)
  (Rendering|SetVisibility (Variables|Default|GetFunction%20Radius%20Sphere_0) true false))

(event EventDisableGradient
  (|CallParentFunction)
  (Rendering|SetVisibility (Variables|Default|GetFunction%20Radius%20Sphere_0) false false))

(fn ConstructionScript
  (|CallParentFunction))

(fn SetBaseMaterial
  (params (Material :type Material%20Interface%20Object%20Reference))
  (Rendering|Material|SetMaterial (Variables|Default|GetGround%20Mesh) 1 Material))

(fn SetFunctionRadius
  (params (%20 :type Float%20%28single-precision%29))
  (bind _returnvalue (/ %20 5e+01))
  (Transformation|SetRelativeScale3D (Variables|Default|GetFunction%20Radius%20Sphere_0) (Math|Vector|MakeVector _returnvalue _returnvalue _returnvalue))
  (Components|Sphere|SetSphereRadius (Variables|Default|GetFunction%20Radius%20Collision) %20 true))

(fn SetPreviousTile
  (params (Previous%20Tile :type Tile%20BP%20Class%20Reference))
  (bind _dockchild (Variables|Default|GetDockChild))
  (bind _output_get (Variables|Default|SetPrevious%20Tile Previous%20Tile))
  (if (.bDock (Utilities|GetClassDefaults _output_get))
    (Rendering|SetVisibility (Variables|Default|GetGround%20Mesh) false false)
    (ChildActorComponent|SetChildActorClass _dockchild _output_get)
    (bind _astile_bp (Utilities|Casting|CastToTile_BP (Variables|/Script/Engine.ChildActorComponent|GetChildActor _dockchild)))
    (Collision|SetCollisionEnabled (Variables|/Game/BP/Tile_BP.Tile_BP_C|GetBox _astile_bp) "NoCollision")))

(fn Upgrade)