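; MG_BP is the machine gun turret player tile, supplying MG-specific data and animation hooks.
; InitDataTable loads the "MG" row of TurretPropertiesTable into TurretProperties.
; AnimBPData casts the anim instance to MG_Skeleton_AnimBlueprint, optionally writes pitch and yaw, and returns the current values.
; It holds no targeting or firing logic of its own.
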(event EventBeginPlay
  (|CallParentFunction) ; This node is disabled and will not be called.\nDrag off pins to build functionality.
)

(event Collision|EventActorBeginOverlap
  (params (OtherActor :type Actor%20Object%20Reference))
  (|CallParentFunction OtherActor) ; This node is disabled and will not be called.\nDrag off pins to build functionality.
)

(event EventTick
  (params (DeltaSeconds :type Float%20%28single-precision%29))
  (|CallParentFunction DeltaSeconds) ; This node is disabled and will not be called.\nDrag off pins to build functionality.
)

(event EventInitDataTable
  (bind _returnvalue (Utilities|GetDataTableRow "/Game/BP/Tiles/PlayerTiles/TurretPropertiesTable.TurretPropertiesTable" "MG")
    (:then
      (Variables|Default|SetTurret%20Properties _returnvalue))))

(fn ConstructionScript
  (|CallParentFunction))

(fn AnimBPData
  (params (Anim%20Instance :type Anim%20Instance%20Object%20Reference) (Set%20Values :type Boolean) (Set%20Yaw :type Float%20%28single-precision%29) (Set%20Pitch :type Float%20%28single-precision%29))
  (bind _asmg_skeleton_anim_blueprint (Utilities|Casting|CastToMG_Skeleton_AnimBlueprint Anim%20Instance))
  (if Set%20Values
    (Variables|/Game/Mesh/Buildings/MachineGun/MG_Skeleton_AnimBlueprint.MG_Skeleton_AnimBlueprint_C|SetPitch _asmg_skeleton_anim_blueprint Set%20Pitch)
    (Variables|/Game/Mesh/Buildings/MachineGun/MG_Skeleton_AnimBlueprint.MG_Skeleton_AnimBlueprint_C|SetYaw _asmg_skeleton_anim_blueprint Set%20Yaw))
  (return (Variables|/Game/Mesh/Buildings/MachineGun/MG_Skeleton_AnimBlueprint.MG_Skeleton_AnimBlueprint_C|GetYaw _asmg_skeleton_anim_blueprint) (Variables|/Game/Mesh/Buildings/MachineGun/MG_Skeleton_AnimBlueprint.MG_Skeleton_AnimBlueprint_C|GetPitch _asmg_skeleton_anim_blueprint)))