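; Scout turret Blueprint, a player tile that supplies the Scout-specific data and animation hookup to inherited turret logic.
; InitDataTable loads the "Scout" row of TurretPropertiesTable into TurretProperties.
; AnimBPData casts the given anim instance to Scout_Anim_BP, optionally writes Yaw and Pitch, and always returns both values.
; The construction script only calls the parent, and the default event stubs are disabled.
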(event EventBeginPlay
  (|CallParentFunction) ; This node is disabled and will not be called.\nDrag off pins to build functionality.
)

(event Collision|EventActorBeginOverlap
  (params (OtherActor :type Actor%20Object%20Reference))
  (|CallParentFunction OtherActor) ; This node is disabled and will not be called.\nDrag off pins to build functionality.
)

(event EventTick
  (params (DeltaSeconds :type Float%20%28single-precision%29))
  (|CallParentFunction DeltaSeconds) ; This node is disabled and will not be called.\nDrag off pins to build functionality.
)

(event EventInitDataTable
  (bind _returnvalue (Utilities|GetDataTableRow "/Game/BP/Tiles/PlayerTiles/TurretPropertiesTable.TurretPropertiesTable" "Scout")
    (:then
      (Variables|Default|SetTurret%20Properties _returnvalue))))

(fn ConstructionScript
  (|CallParentFunction))

(fn AnimBPData
  (params (Anim%20Instance :type Anim%20Instance%20Object%20Reference) (Set%20Values :type Boolean) (Set%20Yaw :type Float%20%28single-precision%29) (Set%20Pitch :type Float%20%28single-precision%29))
  (bind _asscout_anim_bp (Utilities|Casting|CastToScout_Anim_BP Anim%20Instance))
  (if Set%20Values
    (Variables|/Game/Mesh/Buildings/Scout/Scout_Anim_BP.Scout_Anim_BP_C|SetYaw _asscout_anim_bp Set%20Yaw)
    (Variables|/Game/Mesh/Buildings/Scout/Scout_Anim_BP.Scout_Anim_BP_C|SetPitch _asscout_anim_bp Set%20Pitch))
  (return (Variables|/Game/Mesh/Buildings/Scout/Scout_Anim_BP.Scout_Anim_BP_C|GetYaw _asscout_anim_bp) (Variables|/Game/Mesh/Buildings/Scout/Scout_Anim_BP.Scout_Anim_BP_C|GetPitch _asscout_anim_bp)))