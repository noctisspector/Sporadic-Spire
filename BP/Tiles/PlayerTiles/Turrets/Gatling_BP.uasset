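; Gatling turret tile that builds on a parent turret class, supplying its own stats and animation hookup.
; Its properties load from the Gatling row of the turret properties data table.
; Tick watches HasTarget and uses paired DoOnce gates to set the anim Blueprint's Firing flag only when targeting changes.
; AnimBPData optionally writes yaw and pitch to the Gatling anim Blueprint and returns the current values.
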(event EventBeginPlay
  (|CallParentFunction) ; This node is disabled and will not be called.\nDrag off pins to build functionality.
)

(event Collision|EventActorBeginOverlap
  (params (OtherActor :type Actor%20Object%20Reference))
  (|CallParentFunction OtherActor) ; This node is disabled and will not be called.\nDrag off pins to build functionality.
)

(event EventTick
  (params (DeltaSeconds :type Float%20%28single-precision%29))
  (bind _skeletalmesh (Variables|Default|GetSkeletalMesh))
  (bind _returnvalue (Components|SkeletalMesh|GetAnimInstance _skeletalmesh))
  (bind _asgatling_anim_bp (Utilities|Casting|CastToGatling_Anim_BP _returnvalue))
  (|CallParentFunction DeltaSeconds)
  (if (Variables|Default|GetbHasTarget)
    (Utilities|FlowControl|Sequence
      (:then_0
        (Utilities|FlowControl|DoOnce false :!label _label
          (:Completed
            (Variables|/Game/Mesh/Buildings/Gatling/Gatling_Anim_BP.Gatling_Anim_BP_C|SetbFiring _asgatling_anim_bp true))))
      (:then_1
        (goto _label_2 Reset)))
    (else
      (Utilities|FlowControl|Sequence
        (:then_0
          (Utilities|FlowControl|DoOnce false :!label _label_2
            (:Completed
              (Variables|/Game/Mesh/Buildings/Gatling/Gatling_Anim_BP.Gatling_Anim_BP_C|SetbFiring _asgatling_anim_bp false))))
        (:then_1
          (goto _label Reset))))))

(event EventInitDataTable
  (bind _returnvalue (Utilities|GetDataTableRow "/Game/BP/Tiles/PlayerTiles/TurretPropertiesTable.TurretPropertiesTable" "Gatling")
    (:then
      (Variables|Default|SetTurret%20Properties _returnvalue))))

(fn ConstructionScript
  (|CallParentFunction))

(fn AnimBPData
  (params (Anim%20Instance :type Anim%20Instance%20Object%20Reference) (Set%20Values :type Boolean) (Set%20Yaw :type Float%20%28single-precision%29) (Set%20Pitch :type Float%20%28single-precision%29))
  (bind _asgatling_anim_bp (Utilities|Casting|CastToGatling_Anim_BP Anim%20Instance))
  (if Set%20Values
    (Variables|/Game/Mesh/Buildings/Gatling/Gatling_Anim_BP.Gatling_Anim_BP_C|SetYaw _asgatling_anim_bp Set%20Yaw)
    (Variables|/Game/Mesh/Buildings/Gatling/Gatling_Anim_BP.Gatling_Anim_BP_C|SetPitch _asgatling_anim_bp Set%20Pitch))
  (return (Variables|/Game/Mesh/Buildings/Gatling/Gatling_Anim_BP.Gatling_Anim_BP_C|GetYaw _asgatling_anim_bp) (Variables|/Game/Mesh/Buildings/Gatling/Gatling_Anim_BP.Gatling_Anim_BP_C|GetPitch _asgatling_anim_bp)))