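; Procedurally generates the tile world for a tower-defense-style map at BeginPlay, including the enemy path and both bases.
; Temperature and aridity FastNoise maps select each tile's biome from world-type ranges, then a weighted roll picks the tile.
; A random axis-alternating path is carved from enemy spawn to player base, registering waypoints with the GameMode.
; Main-menu mode temporarily forces the Corruption world type and skips path and bases.
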(event EventBeginPlay
  (bind _self self)
  (bind _min_path_length (Variables|Default|GetMin%20Path%20Length))
  (bind _max_path_length (Variables|Default|GetMax%20Path%20Length))
  (bind _base_min_dimension (Variables|Default|GetBase%20Min%20Dimension))
  (bind _noise_type (Variables|GenerationSettings|GetNoise%20Type))
  (bind _interpolation (Variables|GenerationSettings|GetInterpolation))
  (bind _fractal (Variables|GenerationSettings|GetFractal))
  (bind _base_distance_from_edge (Variables|Default|GetBase%20Distance%20From%20Edge))
  (bind _octaves (Variables|GenerationSettings|GetOctaves))
  (bind _octave_lacunarity (Variables|GenerationSettings|GetOctave%20Lacunarity))
  (bind _octave_gain (Variables|GenerationSettings|GetOctave%20Gain))
  (bind _cellular_jitter (Variables|GenerationSettings|GetCellular%20Jitter))
  (bind _cellular_distance_function (Variables|GenerationSettings|GetCellular%20Distance%20Function))
  (bind _cellular_return_type (Variables|GenerationSettings|GetCellular%20Return%20Type))
  (if (Variables|Default|GetbOverrideSize)
    (Variables|Default|SetWorld%20Size (Variables|Default|GetOverridenSize)))
  ;[1 1 1] Main Menu override
  (if (Variables|Default|GetbMM)
    (Variables|/Game/BP/Global_GI.Global_GI_C|SetWorldType (Utilities|GameInstance) "NewEnumerator4"))
  ;[1 1 1] Generate Seeds
  (Variables|GenerationSettings|SetAridity%20Seed (Math|Random|RandomIntegerinRange 0 99999999))
  (Variables|GenerationSettings|SetAridity%20Seed (Math|Random|RandomIntegerinRange 0 99999999))
  ;[1 1 1] Create Biome Noise
  (bind _returnvalue (Game|ConstructObjectfromClass "/Script/FastNoiseGenerator.FastNoiseWrapper" _self))
  (Variables|Default|SetTemp%20Noise _returnvalue)
  (bind _returnvalue_2 (Game|ConstructObjectfromClass "/Script/FastNoiseGenerator.FastNoiseWrapper" _self))
  (Variables|Default|SetAridity%20Noise _returnvalue_2)
  (Class|FastNoiseWrapper|SetupFastNoise (Variables|Default|GetTemp%20Noise) _noise_type (Variables|GenerationSettings|GetTemp%20Seed) (* (Variables|GenerationSettings|GetFrequency) (Utilities|GetWorldtypePerlinData (Variables|/Game/BP/Global_GI.Global_GI_C|GetWorldType (Utilities|GameInstance)))) _interpolation _fractal _octaves _octave_lacunarity _octave_gain _cellular_jitter _cellular_distance_function _cellular_return_type)
  (Class|FastNoiseWrapper|SetupFastNoise (Variables|Default|GetAridity%20Noise) _noise_type (Variables|GenerationSettings|GetAridity%20Seed) (* (Variables|GenerationSettings|GetFrequency) (Utilities|GetWorldtypePerlinData (Variables|/Game/BP/Global_GI.Global_GI_C|GetWorldType (Utilities|GameInstance)))) _interpolation _fractal _octaves _octave_lacunarity _octave_gain _cellular_jitter _cellular_distance_function _cellular_return_type)
  ;[1 1 1] Loop Though World
  (for _index (range (Utilities|Invert(int) (.rows (Variables|Default|GetWorld%20Size))) (.rows (Variables|Default|GetWorld%20Size)))
    (for _index_2 (range (Utilities|Invert(int) (.columns (Variables|Default|GetWorld%20Size))) (.columns (Variables|Default|GetWorld%20Size)))
      ;[1 1 1] Generate World
      (CallFunction|GenerateTile (Utilities|Struct|MakeWorldPosition _index _index_2))))
  (if (Variables|Default|GetbMM)
    ;[1 1 1] Revert world type if mm
    (Variables|/Game/BP/Global_GI.Global_GI_C|SetWorldType (Utilities|GameInstance) "NewEnumerator0")
    (else
      ;[1 1 1] Generate Start + End
      (while (or (< (Math|Integer|Absolute(Integer) (- (.rows (Variables|Default|GetStart%20Location)) (.rows (Variables|Default|GetEnd%20Location)))) _base_min_dimension) (< (Math|Integer|Absolute(Integer) (- (.columns (Variables|Default|GetStart%20Location)) (.columns (Variables|Default|GetEnd%20Location)))) _base_min_dimension))
        (Variables|Default|SetStart%20Location (Utilities|Struct|MakeWorldPosition (Math|Random|RandomIntegerinRange (Utilities|Invert(int) (- (.rows (Variables|Default|GetWorld%20Size)) _base_distance_from_edge)) (- (.rows (Variables|Default|GetWorld%20Size)) _base_distance_from_edge)) (Math|Random|RandomIntegerinRange (Utilities|Invert(int) (- (.columns (Variables|Default|GetWorld%20Size)) _base_distance_from_edge)) (- (.columns (Variables|Default|GetWorld%20Size)) _base_distance_from_edge))))
        (Variables|Default|SetEnd%20Location (Utilities|Struct|MakeWorldPosition (Math|Random|RandomIntegerinRange (Utilities|Invert(int) (- (.rows (Variables|Default|GetWorld%20Size)) _base_distance_from_edge)) (- (.rows (Variables|Default|GetWorld%20Size)) _base_distance_from_edge)) (Math|Random|RandomIntegerinRange (Utilities|Invert(int) (- (.columns (Variables|Default|GetWorld%20Size)) _base_distance_from_edge)) (- (.columns (Variables|Default|GetWorld%20Size)) _base_distance_from_edge)))))
      ;[1 1 1] Loop Through Path Nodes
      (Variables|Default|SetLatest%20Path%20Gen%20Location%201 (Variables|Default|GetStart%20Location))
      (for _index_3 (range 1 (Variables|Default|GetPath%20Count))
        ;[1 1 1] Find Direction
        (Variables|Default|SetNew%20Direction (select (== (Math|Integer|%(Integer) _index_3 2) 0) (Math|Random|RandomIntegerinRange 0 1) (Math|Random|RandomIntegerinRange 2 3)))
        (while (== (Variables|Default|GetNew%20Direction) (Utilities|InvertDirection (Variables|Default|GetPrevious%20Direction)))
          (Variables|Default|SetNew%20Direction (select (== (Math|Integer|%(Integer) _index_3 2) 0) (Math|Random|RandomIntegerinRange 0 1) (Math|Random|RandomIntegerinRange 2 3))))
        ;[1 1 1] Find New Coords
        (bind ___ (CallFunction|ConverttoRealSpace (Utilities|Add(WorldPosition) (Variables|Default|GetLatest%20Path%20Gen%20Location%201) (Utilities|Select :Index (Variables|Default|GetNew%20Direction) :Option%200 (Utilities|Struct|MakeWorldPosition (Math|Random|RandomIntegerinRange _min_path_length _max_path_length) 0) :Option%201 (Utilities|Struct|MakeWorldPosition (Utilities|Invert(int) (Math|Random|RandomIntegerinRange _min_path_length _max_path_length)) 0) :Option%202 (Utilities|Struct|MakeWorldPosition 0 (Math|Random|RandomIntegerinRange _min_path_length _max_path_length)) :Option%203 (Utilities|Struct|MakeWorldPosition 0 (Utilities|Invert(int) (Math|Random|RandomIntegerinRange _min_path_length _max_path_length)))))))
        (bind _output_get (Variables|Default|SetLatest%20Path%20Gen%20Location%202 ___))
        ;[1 1 1] Fill
        (CallFunction|Fill (Variables|Default|GetLatest%20Path%20Gen%20Location%201) _output_get "/Game/BP/Tiles/PlayerTiles/EnemyPath_BP.EnemyPath_BP_C" true false)
        (CallFunction|SpawnWaypoint _output_get)
        ;[1 1 1] Update Data
        (Variables|Default|SetLatest%20Path%20Gen%20Location%201 _output_get)
        (Variables|Default|SetPrevious%20Direction (Variables|Default|GetNew%20Direction)))
      ;[1 1 1] Finish Path
      (bind _output_get_2 (Variables|Default|SetLatest%20Path%20Gen%20Location%202 (Utilities|Struct|MakeWorldPosition (.rows (Variables|Default|GetEnd%20Location)) (.Columns (Utilities|Struct|BreakWorldPosition (Variables|Default|GetLatest%20Path%20Gen%20Location%201))))))
      (CallFunction|Fill (Variables|Default|GetLatest%20Path%20Gen%20Location%201) _output_get_2 "/Game/BP/Tiles/PlayerTiles/EnemyPath_BP.EnemyPath_BP_C" false false)
      (CallFunction|SpawnWaypoint _output_get_2)
      (Variables|Default|SetLatest%20Path%20Gen%20Location%201 _output_get_2)
      (bind _output_get_3 (Variables|Default|SetLatest%20Path%20Gen%20Location%202 (Utilities|Struct|MakeWorldPosition (.Rows (Utilities|Struct|BreakWorldPosition (Variables|Default|GetLatest%20Path%20Gen%20Location%201))) (.columns (Variables|Default|GetEnd%20Location)))))
      (CallFunction|Fill (Variables|Default|GetLatest%20Path%20Gen%20Location%201) _output_get_3 "/Game/BP/Tiles/PlayerTiles/EnemyPath_BP.EnemyPath_BP_C" false false)
      (CallFunction|SpawnWaypoint _output_get_3)
      (Variables|Default|SetLatest%20Path%20Gen%20Location%201 _output_get_3)
      ;[1 1 1] Generate Bases
      (Utilities|ReplaceTile (Variables|Default|GetStart%20Location) "/Game/BP/Tiles/PlayerTiles/EnemySpawn_BP.EnemySpawn_BP_C")
      (Utilities|ReplaceTile (Variables|Default|GetEnd%20Location) "/Game/BP/Tiles/PlayerTiles/PlayerBase_BP.PlayerBase_BP_C"))))

(fn ConstructionScript)

(fn GenerateTile
  (params (World%20Position :type World%20Position%20Structure))
  (bind (_rows _columns) (Utilities|Struct|BreakWorldPosition World%20Position))
  (bind (_rows_2 _columns_2) (Utilities|Struct|BreakWorldPosition World%20Position))
  (bind _returnvalue (Math|Conversions|ToFloat(Integer) _columns))
  (bind _returnvalue_2 (Math|Conversions|ToFloat(Integer) _rows))
  (Variables|/Game/BP/Global_GI.Global_GI_C|SetRoot%20Position (Utilities|GameInstance) (Transformation|GetActorLocation))
  ;[1 1 1] Get Noise Values
  (bind _returnvalue_3 (Class|FastNoiseWrapper|GetNoise2D (Variables|Default|GetTemp%20Noise) _returnvalue_2 _returnvalue))
  (bind _returnvalue_4 (Class|FastNoiseWrapper|GetNoise2D (Variables|Default|GetAridity%20Noise) _returnvalue_2 _returnvalue))
  (bind _biome (CallFunction|GenerateBiome _returnvalue_3 _returnvalue_4))
  (bind _tile (CallFunction|BiometoTile _biome))
  ;[1 1 1] Spawn Tile
  (bind _returnvalue_5 (Game|SpawnActorfromClass _tile (Math|Transform|MakeTransform (+ (Transformation|GetActorLocation) (* (Math|Vector|MakeVector (Math|Conversions|ToFloat(Integer) _rows_2) (Math|Conversions|ToFloat(Integer) _columns_2) 0.0) (Utilities|TileSize))) "0, 0, 0" "1,1,1") "Undefined" 0 0))
  (bind _astile_bp (Utilities|Casting|CastToTile_BP _returnvalue_5))
  (Variables|/Game/BP/Tile_BP.Tile_BP_C|SetWorld%20Position _astile_bp World%20Position))

(fn GenerateBiome
  (params (Temp :type Float%20%28single-precision%29) (Aridity :type Float%20%28single-precision%29))
  (for _array_element (Variables|Default|GetBiomes)
    (CallFunction|SetChosenBiome (Math|Vector2D|MakeVector2D (/ (+ Temp 1.0) 2.0) (/ (+ Aridity 1.0) 2.0)) _array_element))
  (return (Variables|Default|GetChosen%20Biome)))

(fn BiometoTile
  (params (Biome :type Biome%20BP%20Class%20Reference))
  (bind _distribution (Utilities|GetClassDefaults Biome))
  ;[1 1 1] Calculate Sum
  (for _array_element _distribution
    (LocalVariables|SetWeight%20Sum (+ (.weight _array_element) (LocalVariables|GetWeight%20Sum))))
  ;[1 1 1] Get Random Number
  (LocalVariables|SetRandom%20Float (* (Math|Random|RandomFloat) (LocalVariables|GetWeight%20Sum)))
  (for _array_element_2 _distribution
    (if (< (LocalVariables|GetRandom%20Float) (.weight _array_element_2))
      (return (.tile _array_element_2))
      (else
        (LocalVariables|SetRandom%20Float (- (LocalVariables|GetRandom%20Float) (.weight _array_element_2))))))
  (return "/Game/BP/Tiles/PlayerTiles/YellowDebugPath_BP.YellowDebugPath_BP_C"))

(fn SetChosenBiome
  (params (Temp/Arid :type Vector%202D%20Structure) (InputPin :type Biome%20BP%20Class%20Reference))
  (bind __ (Utilities|IfValuesinBiome InputPin Temp/Arid)
    (:OutputPin
      (if __
        (Variables|Default|SetChosen%20Biome InputPin)))))

(fn Fill
  (params (Position%201 :type World%20Position%20Structure%20%28by%20ref%29) (Position%202 :type World%20Position%20Structure%20%28by%20ref%29) (Tile :type Tile%20BP%20Class%20Reference) (Skip%20Start :type Boolean) (Skip%20End :type Boolean))
  (bind (_rows _columns) (Utilities|Struct|BreakWorldPosition Position%201))
  (bind (_rows_2 _columns_2) (Utilities|Struct|BreakWorldPosition Position%202))
  (bind _world_size (Variables|Default|GetWorld%20Size))
  (if (> _rows _rows_2)
    (LocalVariables|SetNew%20Position%201 (Utilities|Struct|MakeWorldPosition _rows_2 (.columns (LocalVariables|GetNew%20Position%201))))
    (LocalVariables|SetNew%20Position%202 (Utilities|Struct|MakeWorldPosition _rows (.columns (LocalVariables|GetNew%20Position%202))))
    (else
      (LocalVariables|SetNew%20Position%201 (Utilities|Struct|MakeWorldPosition _rows (.columns (LocalVariables|GetNew%20Position%201))))
      (LocalVariables|SetNew%20Position%202 (Utilities|Struct|MakeWorldPosition _rows_2 (.columns (LocalVariables|GetNew%20Position%202))))))
  (if (> _columns _columns_2)
    (LocalVariables|SetNew%20Position%201 (Utilities|Struct|MakeWorldPosition (.rows (LocalVariables|GetNew%20Position%201)) _columns_2))
    (LocalVariables|SetNew%20Position%202 (Utilities|Struct|MakeWorldPosition (.rows (LocalVariables|GetNew%20Position%202)) _columns))
    (else
      (LocalVariables|SetNew%20Position%201 (Utilities|Struct|MakeWorldPosition (.rows (LocalVariables|GetNew%20Position%201)) _columns))
      (LocalVariables|SetNew%20Position%202 (Utilities|Struct|MakeWorldPosition (.rows (LocalVariables|GetNew%20Position%202)) _columns_2))))
  (LocalVariables|SetLast%20Position (Utilities|Struct|MakeWorldPosition (select Skip%20End (select (== (.Rows (Utilities|Struct|BreakWorldPosition (LocalVariables|GetNew%20Position%201))) (.Rows (Utilities|Struct|BreakWorldPosition (LocalVariables|GetNew%20Position%202)))) (.Rows (Utilities|Struct|BreakWorldPosition (LocalVariables|GetNew%20Position%202))) (+ (.Rows (Utilities|Struct|BreakWorldPosition (LocalVariables|GetNew%20Position%202))) -1)) (.Rows (Utilities|Struct|BreakWorldPosition (LocalVariables|GetNew%20Position%202)))) (select Skip%20End (select (== (.Columns (Utilities|Struct|BreakWorldPosition (LocalVariables|GetNew%20Position%201))) (.Columns (Utilities|Struct|BreakWorldPosition (LocalVariables|GetNew%20Position%202)))) (.Columns (Utilities|Struct|BreakWorldPosition (LocalVariables|GetNew%20Position%202))) (+ (.Columns (Utilities|Struct|BreakWorldPosition (LocalVariables|GetNew%20Position%202))) -1)) (.Columns (Utilities|Struct|BreakWorldPosition (LocalVariables|GetNew%20Position%202))))))
  (for _index (range (select Skip%20Start (select (== (.Rows (Utilities|Struct|BreakWorldPosition (LocalVariables|GetNew%20Position%201))) (.Rows (Utilities|Struct|BreakWorldPosition (LocalVariables|GetNew%20Position%202)))) (.Rows (Utilities|Struct|BreakWorldPosition (LocalVariables|GetNew%20Position%201))) (+ (.Rows (Utilities|Struct|BreakWorldPosition (LocalVariables|GetNew%20Position%201))) 1)) (.Rows (Utilities|Struct|BreakWorldPosition (LocalVariables|GetNew%20Position%201)))) (select Skip%20End (select (== (.Rows (Utilities|Struct|BreakWorldPosition (LocalVariables|GetNew%20Position%201))) (.Rows (Utilities|Struct|BreakWorldPosition (LocalVariables|GetNew%20Position%202)))) (.Rows (Utilities|Struct|BreakWorldPosition (LocalVariables|GetNew%20Position%202))) (+ (.Rows (Utilities|Struct|BreakWorldPosition (LocalVariables|GetNew%20Position%202))) -1)) (.Rows (Utilities|Struct|BreakWorldPosition (LocalVariables|GetNew%20Position%202)))))
    (for _index_2 (range (select Skip%20Start (select (== (.Columns (Utilities|Struct|BreakWorldPosition (LocalVariables|GetNew%20Position%201))) (.Columns (Utilities|Struct|BreakWorldPosition (LocalVariables|GetNew%20Position%202)))) (.Columns (Utilities|Struct|BreakWorldPosition (LocalVariables|GetNew%20Position%201))) (+ (.Columns (Utilities|Struct|BreakWorldPosition (LocalVariables|GetNew%20Position%201))) 1)) (.Columns (Utilities|Struct|BreakWorldPosition (LocalVariables|GetNew%20Position%201)))) (select Skip%20End (select (== (.Columns (Utilities|Struct|BreakWorldPosition (LocalVariables|GetNew%20Position%201))) (.Columns (Utilities|Struct|BreakWorldPosition (LocalVariables|GetNew%20Position%202)))) (.Columns (Utilities|Struct|BreakWorldPosition (LocalVariables|GetNew%20Position%202))) (+ (.Columns (Utilities|Struct|BreakWorldPosition (LocalVariables|GetNew%20Position%202))) -1)) (.Columns (Utilities|Struct|BreakWorldPosition (LocalVariables|GetNew%20Position%202)))))
      (if (Math|Boolean|ANDBoolean (>= _index (Utilities|Invert(int) (.rows _world_size))) (<= _index (.rows _world_size)) (>= _index_2 (Utilities|Invert(int) (.columns _world_size))) (<= _index_2 (.columns _world_size)))
        (bind _new_tile_ref (Utilities|ReplaceTile (Utilities|Struct|MakeWorldPosition _index _index_2) Tile))
        (if (and (== _index (.rows (LocalVariables|GetLast%20Position))) (== (.columns (LocalVariables|GetLast%20Position)) _index_2))
          (LocalVariables|SetLast%20Tile _new_tile_ref)))))
  (return (LocalVariables|GetLast%20Tile)))

(fn ConverttoRealSpace
  (params (%20 :type World%20Position%20Structure))
  (bind _world_size (Variables|Default|GetWorld%20Size))
  (bind ___ (Utilities|Invert(int) (.rows _world_size)))
  (bind ____2 (Utilities|Invert(int) (.columns _world_size)))
  (bind _output_get (LocalVariables|SetReturn %20))
  (if (< (.rows _output_get) ___)
    (LocalVariables|SetReturn (Utilities|Struct|MakeWorldPosition ___ (.Columns (Utilities|Struct|BreakWorldPosition (LocalVariables|GetReturn))))))
  (if (> (.rows _output_get) (.rows _world_size))
    (LocalVariables|SetReturn (Utilities|Struct|MakeWorldPosition (.rows _world_size) (.Columns (Utilities|Struct|BreakWorldPosition (LocalVariables|GetReturn))))))
  (if (< (.columns _output_get) ____2)
    (LocalVariables|SetReturn (Utilities|Struct|MakeWorldPosition (.Rows (Utilities|Struct|BreakWorldPosition (LocalVariables|GetReturn))) ____2)))
  (if (> (.columns _output_get) (.columns _world_size))
    (LocalVariables|SetReturn (Utilities|Struct|MakeWorldPosition (.Rows (Utilities|Struct|BreakWorldPosition (LocalVariables|GetReturn))) (.columns _world_size))))
  (return (LocalVariables|GetReturn)))

(fn SpawnWaypoint
  (params (Location :type World%20Position%20Structure))
  (bind (_rows _columns) (Utilities|Struct|BreakWorldPosition Location))
  (bind _waypoint_index (Variables|Default|GetWaypoint%20Index))
  (bind _returnvalue (Game|SpawnActorfromClass "/Game/BP/WayPoint_BP.WayPoint_BP_C" (Math|Transform|MakeTransform (+ (Transformation|GetActorLocation) (* (Math|Vector|MakeVector (Math|Conversions|ToFloat(Integer) _rows) (Math|Conversions|ToFloat(Integer) _columns) 0.65) (Utilities|TileSize))) "0, 0, 0" "1,1,1") "Undefined" 0 0))
  (Variables|/Game/BP/WayPoint_BP.WayPoint_BP_C|SetIndex _returnvalue _waypoint_index)
  (Default|AddWaypoint (Utilities|Gamemode) _returnvalue)
  (Math|Integer|IncrementInt _waypoint_index))