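; Tile actor that provides visual highlighting and a radius preview for other code to drive.
; Separate gradient and hover-gradient components are shown with a caller-supplied material or hidden, each tracking a boolean state.
; The main gradient is disabled on BeginPlay.
; Radius preview shows a sphere component scaled uniformly from the given radius divided by 50, with a matching function to hide it.
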(event EventBeginPlay
  (CallFunction|DisableGradient))

(fn ConstructionScript)

(fn EnableGradient
  (params (Material :type Material%20Interface%20Object%20Reference))
  (Rendering|Material|SetMaterial (Variables|Default|GetGradient) 0 Material)
  (Rendering|SetVisibility (Variables|Default|GetGradient) true false)
  (Variables|Default|SetbGradient true))

(fn DisableGradient
  (Rendering|SetVisibility (Variables|Default|GetGradient) false false)
  (Variables|Default|SetbGradient false))

(fn EnableHoverGradient
  (params (Material :type Material%20Interface%20Object%20Reference))
  (bind _hovergradient (Variables|Default|GetHoverGradient))
  (Rendering|Material|SetMaterial _hovergradient 0 Material)
  (Rendering|SetVisibility _hovergradient true false)
  (Variables|Default|SetbHoverGradient true))

(fn DisableHoverGradient
  (Rendering|SetVisibility (Variables|Default|GetHoverGradient) false false)
  (Variables|Default|SetbHoverGradient false))

(fn PreviewRadius
  (params (Radius :type Float%20%28single-precision%29))
  (bind _returnvalue (/ Radius 5e+01))
  (bind _function_radius_sphere (Variables|Default|GetFunction%20Radius%20Sphere))
  (Rendering|SetVisibility _function_radius_sphere true false)
  (Transformation|SetRelativeScale3D _function_radius_sphere (Math|Vector|MakeVector _returnvalue _returnvalue _returnvalue)))

(fn StopPreviewingRadius
  (Rendering|SetVisibility (Variables|Default|GetFunction%20Radius%20Sphere) false false))