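; Music controller Blueprint that plays its audio component's music repeatedly with randomized pauses between plays.
; On BeginPlay it waits a random delay, activates the audio component, and binds its finished event.
; Each time the audio finishes, it waits again and replays from the start.
; The Random Delay macro draws the wait time from the SongDelay vector's range.
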(event Custom|Song%20Finished
  (Utilities|RandomDelay)
  (Audio|Components|Audio|Play (Variables|Default|GetAudio) 0.0))

(event EventBeginPlay
  (bind _audio (Variables|Default|GetAudio))
  (Utilities|RandomDelay)
  (Components|Activation|Activate _audio false)
  (EventDispatchers|AssignOnAudioFinished _audio (delegate Custom|Song%20Finished)))

(fn ConstructionScript)