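; Tesla projectile Blueprint that acts as an instant-hit beam attack on a target instead of flying to it.
; BeginPlay spawns a beam particle and pins its source to the projectile's location.
; SetDefaultValues extends the parent's setup, aims the beam at the target, immediately applies knockback, damage and stun, spawns the explosion effect there, then destroys the actor.
; The sphere overlap event is left empty, so collision plays no part in hits.
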(event OnComponentBeginOverlap(Sphere)
  (params (OverlappedComponent :type Primitive%20Component%20Object%20Reference) (OtherActor :type Actor%20Object%20Reference) (OtherComp :type Primitive%20Component%20Object%20Reference) (OtherBodyIndex :type Integer) (bFromSweep :type Boolean) (SweepResult :type Hit%20Result%20Structure%20%28by%20ref%29)))

(event EventBeginPlay
  (bind _returnvalue (Transformation|GetActorLocation))
  (|CallParentFunction)
  (bind _returnvalue_2 (Effects|SpawnEmitteratLocation "/Game/Particle/TeslaBeam_P.TeslaBeam_P" _returnvalue (Transformation|GetActorRotation)))
  (bind _output_get (Variables|Default|SetBeam%20F _returnvalue_2))
  (Class|ParticleSystemComponent|SetBeamSourcePoint _returnvalue_2 0 _returnvalue))

(event EventSetDefaultValues
  (params (Projectile%20Speed :type Float%20%28single-precision%29) (Explosion%20Effect :type Particle%20System%20Object%20Reference) (Damage :type Float%20%28single-precision%29) (Knockback :type Float%20%28single-precision%29) (Damage%20Radius :type Float%20%28single-precision%29) (target :type Enemy%20BP%20Object%20Reference) (Stun%20Time :type Float%20%28single-precision%29) (Poison :type Float%20%28single-precision%29) (Poison%20Duration :type Integer) (Poison%20Effect :type Particle%20System%20Object%20Reference) (Exp%20Sound :type Sound%20Base%20Object%20Reference))
  (bind _returnvalue (Transformation|GetActorLocation (Variables|Default|Gettarget)))
  (|CallParentFunction Projectile%20Speed Explosion%20Effect Damage Knockback Damage%20Radius target Stun%20Time 0.0 0 0 0)
  (Class|ParticleSystemComponent|SetBeamTargetPoint (Variables|Default|GetBeam%20F) 0 _returnvalue)
  (Default|SetKnockback (Variables|Default|Gettarget) (Variables|Default|GetKnockback) (Transformation|GetActorRotation))
  (Default|Damage (Variables|Default|Gettarget) (Variables|Default|GetDamage))
  (Default|Stun (Variables|Default|Gettarget) (Variables|Default|GetStun%20Time))
  (Effects|SpawnEmitteratLocation (Variables|Default|GetExplosion%20Effect) _returnvalue)
  (Actor|DestroyActor))

(event EventTick
  (params (DeltaSeconds :type Float%20%28single-precision%29))
  (|CallParentFunction DeltaSeconds) ; This node is disabled and will not be called.\nDrag off pins to build functionality.
)

(fn ConstructionScript
  (|CallParentFunction))