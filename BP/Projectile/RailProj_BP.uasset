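; RailProj_BP is a railgun projectile that damages and knocks back enemies it overlaps.
; On BeginPlay it spawns the Beam_P emitter at its location and rotation.
; Sphere overlaps with Enemy_BP actors apply Knockback along the projectile's rotation, then Damage.
; Each enemy hit is stored in HitActors and checked by IsUniqueEnemy, so the projectile affects each enemy only once.
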(event OnComponentBeginOverlap(Sphere)
  (params (OverlappedComponent :type Primitive%20Component%20Object%20Reference) (OtherActor :type Actor%20Object%20Reference) (OtherComp :type Primitive%20Component%20Object%20Reference) (OtherBodyIndex :type Integer) (bFromSweep :type Boolean) (SweepResult :type Hit%20Result%20Structure%20%28by%20ref%29))
  (bind _asenemy_bp (Utilities|Casting|CastToEnemy_BP OtherActor))
  (bind _unique (CallFunction|IsUniqueEnemy _asenemy_bp))
  (if _unique
    (Default|SetKnockback _asenemy_bp (Variables|Default|GetKnockback) (Transformation|GetActorRotation))
    (Default|Damage _asenemy_bp (Variables|Default|GetDamage))
    (Utilities|FlowControl|Sequence
      (:then_1
        (Utilities|Array|Add (Variables|Default|GetHit%20Actors) _asenemy_bp)))))

(event EventBeginPlay
  (|CallParentFunction)
  (Effects|SpawnEmitteratLocation "/Game/Particle/Beam_P.Beam_P" (Transformation|GetActorLocation) (Transformation|GetActorRotation)))

(event EventTick
  (params (DeltaSeconds :type Float%20%28single-precision%29))
  (|CallParentFunction DeltaSeconds) ; This node is disabled and will not be called.\nDrag off pins to build functionality.
)

(fn ConstructionScript
  (|CallParentFunction))

(fn IsUniqueEnemy
  (params (Enemy :type Enemy%20BP%20Object%20Reference))
  (LocalVariables|SetbUnique true)
  (for _array_element (Variables|Default|GetHit%20Actors)
    (if (== Enemy _array_element)
      (LocalVariables|SetbUnique false)))
  (return (LocalVariables|GetbUnique)))