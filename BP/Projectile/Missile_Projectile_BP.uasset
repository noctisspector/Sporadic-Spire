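; Missile projectile Blueprint that homes in on a target, building on a parent projectile class.
; When its default values are set, it calls the parent, then adds a static mesh component to the target and assigns it as the projectile movement's homing target.
; Each tick it checks the target and switches homing off once the target is dead or invalid.
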(event EventBeginPlay
  (|CallParentFunction) ; This node is disabled and will not be called.\nDrag off pins to build functionality.
)

(event Collision|EventActorBeginOverlap
  (params (OtherActor :type Actor%20Object%20Reference))
  (|CallParentFunction OtherActor) ; This node is disabled and will not be called.\nDrag off pins to build functionality.
)

(event EventTick
  (params (DeltaSeconds :type Float%20%28single-precision%29))
  (bind _target (Variables|Default|Gettarget))
  (|CallParentFunction DeltaSeconds)
  (Utilities|IsValid _target
    (:Is%20Valid
      (if (Variables|/Game/BP/Enemy/Enemy_BP.Enemy_BP_C|GetbDead _target)
        (Utilities|FlowControl|DoOnce false :!label _label
          (:Completed
            (Variables|/Script/Engine.ProjectileMovementComponent|SetbIsHomingProjectile (Variables|Default|GetProjectileMovement) false)))))
    (:Is%20Not%20Valid
      (goto _label))))

(event EventSetDefaultValues
  (params (Projectile%20Speed :type Float%20%28single-precision%29) (Explosion%20Effect :type Particle%20System%20Object%20Reference) (Damage :type Float%20%28single-precision%29) (Knockback :type Float%20%28single-precision%29) (Damage%20Radius :type Float%20%28single-precision%29) (target :type Enemy%20BP%20Object%20Reference) (Stun%20Time :type Float%20%28single-precision%29) (Poison :type Float%20%28single-precision%29) (Poison%20Duration :type Integer) (Poison%20Effect :type Particle%20System%20Object%20Reference) (Exp%20Sound :type Sound%20Base%20Object%20Reference))
  (|CallParentFunction Projectile%20Speed Explosion%20Effect Damage Knockback Damage%20Radius target Stun%20Time Poison Poison%20Duration Poison%20Effect Exp%20Sound)
  (bind _returnvalue (AddComponent|AddStaticMeshComponent target false))
  (Utilities|IsValid _returnvalue
    (:Is%20Valid
      (Variables|/Script/Engine.ProjectileMovementComponent|SetHomingTargetComponent (Variables|Default|GetProjectileMovement) _returnvalue))))

(fn ConstructionScript
  (|CallParentFunction))