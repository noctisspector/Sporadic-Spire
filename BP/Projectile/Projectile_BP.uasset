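; Configurable projectile actor that damages, knocks back, stuns and poisons the Enemy_BP it overlaps, and self-destructs after a timeout.
; SetDefaultValues scales movement velocity and stores the combat stats and effects.
; Sphere begin and end overlaps share CollisionMacro, which applies the hit, then explodes with particles and sound.
; A positive radius adds curve-scaled damage, outward knockback and stun, but no poison, to nearby enemies via an all-actor distance check.
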(event OnComponentBeginOverlap(Sphere)
  (params (OverlappedComponent :type Primitive%20Component%20Object%20Reference) (OtherActor :type Actor%20Object%20Reference) (OtherComp :type Primitive%20Component%20Object%20Reference) (OtherBodyIndex :type Integer) (bFromSweep :type Boolean) (SweepResult :type Hit%20Result%20Structure%20%28by%20ref%29))
  (Utilities|CollisionMacro OtherActor))

(event OnComponentEndOverlap(Sphere)
  (params (OverlappedComponent :type Primitive%20Component%20Object%20Reference) (OtherActor :type Actor%20Object%20Reference) (OtherComp :type Primitive%20Component%20Object%20Reference) (OtherBodyIndex :type Integer))
  (Utilities|CollisionMacro OtherActor))

(event EventBeginPlay
  (Utilities|FlowControl|Delay 25.0)
  (Actor|DestroyActor))

(event Collision|EventActorBeginOverlap
  (params (OtherActor :type Actor%20Object%20Reference)))

(event EventTick
  (params (DeltaSeconds :type Float%20%28single-precision%29)))

(fn ConstructionScript)

(fn SetDefaultValues
  (params (Projectile%20Speed :type Float%20%28single-precision%29) (Explosion%20Effect :type Particle%20System%20Object%20Reference) (Damage :type Float%20%28single-precision%29) (Knockback :type Float%20%28single-precision%29) (Damage%20Radius :type Float%20%28single-precision%29) (target :type Enemy%20BP%20Object%20Reference) (Stun%20Time :type Float%20%28single-precision%29) (Poison :type Float%20%28single-precision%29) (Poison%20Duration :type Integer) (Poison%20Effect :type Particle%20System%20Object%20Reference) (Exp%20Sound :type Sound%20Base%20Object%20Reference))
  (bind _projectilemovement (Variables|Default|GetProjectileMovement))
  (Variables|/Script/Engine.MovementComponent|SetVelocity _projectilemovement (* (Variables|/Script/Engine.MovementComponent|GetVelocity _projectilemovement) Projectile%20Speed))
  (Variables|Default|SetDamage Damage)
  (Variables|Default|SetKnockback Knockback)
  (Variables|Default|SetExplosion%20Effect Explosion%20Effect)
  (Variables|Default|SetDamage%20Radius Damage%20Radius)
  (Variables|Default|Settarget target)
  (Variables|Default|SetStun%20Time Stun%20Time)
  (Variables|Default|SetPoison Poison)
  (Variables|Default|SetPoison%20Duration Poison%20Duration)
  (Variables|Default|SetPoison%20Effect Poison%20Effect)
  (Variables|Default|SetExp%20Sound Exp%20Sound))

(fn ExpSoundFunction
  (Audio|PlaySoundatLocation (Variables|Default|GetExp%20Sound) (Transformation|GetActorLocation) "0, 0, 0" 1.0 1.0 0.0 "/Game/Sounds/SFX_Att.SFX_Att" "/Game/Sounds/SFX_Con.SFX_Con" 0))