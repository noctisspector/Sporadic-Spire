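; Lightning consumable projectile that detonates in an area-of-effect blast when its sphere overlaps an enemy or a non-turret tile.
; The blast checks all Enemy_BP actors within DamageRadius, applying outward knockback, a stun, and damage scaled by a distance-based curve.
; It then spawns explosion and lightning beam particles, plays the explosion sound and destroys itself.
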(event OnComponentBeginOverlap(Sphere)
  (params (OverlappedComponent :type Primitive%20Component%20Object%20Reference) (OtherActor :type Actor%20Object%20Reference) (OtherComp :type Primitive%20Component%20Object%20Reference) (OtherBodyIndex :type Integer) (bFromSweep :type Boolean) (SweepResult :type Hit%20Result%20Structure%20%28by%20ref%29))
  (bind _returnvalue (Transformation|GetActorLocation))
  (bind _damage_radius (Variables|Default|GetDamage%20Radius))
  (Utilities|Casting|CastToEnemy_BP OtherActor
    (:then
      _)
    (:CastFailed
      (Utilities|Casting|CastToTile_BP OtherActor)
      (Utilities|Casting|CastToTurret_BP OtherActor
        (:CastFailed
          _))))
  (bind _outactors (Actor|GetAllActorsOfClass "/Game/BP/Enemy/Enemy_BP.Enemy_BP_C"))
  (for _array_element _outactors
    (if (<= (Transformation|GetDistanceTo _array_element) _damage_radius)
      (Default|SetKnockback _array_element (Variables|Default|GetKnockback) (Math|Rotator|FindLookatRotation (Transformation|GetActorLocation) (Transformation|GetActorLocation _array_element)))
      (Default|Damage _array_element (* (Math|Curves|GetFloatValue (Variables|Default|GetDamage%20Curve) (/ (Transformation|GetDistanceTo _array_element) _damage_radius)) (Variables|Default|GetDamage)))
      (Default|Stun _array_element (Variables|Default|GetStun%20Time))))
  (Effects|SpawnEmitteratLocation (Variables|Default|GetExplosion%20Effect) _returnvalue)
  (Effects|SpawnEmitteratLocation "/Game/Particle/LightningBeam_P.LightningBeam_P" _returnvalue)
  (CallFunction|ExpSoundFunction)
  (Actor|DestroyActor))

(event EventBeginPlay
  (|CallParentFunction) ; This node is disabled and will not be called.\nDrag off pins to build functionality.
)

(event Collision|EventActorBeginOverlap
  (params (OtherActor :type Actor%20Object%20Reference))
  (|CallParentFunction OtherActor) ; This node is disabled and will not be called.\nDrag off pins to build functionality.
)

(event EventTick
  (params (DeltaSeconds :type Float%20%28single-precision%29))
  (|CallParentFunction DeltaSeconds) ; This node is disabled and will not be called.\nDrag off pins to build functionality.
)

(fn ConstructionScript
  (|CallParentFunction))