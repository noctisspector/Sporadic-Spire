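; Player pawn for a tile-based tower defense game, handling camera pan and zoom, money and gold, menus and cheat inputs.
; A cursor trace feeds tile hover, radius previews and clicks, which branch on ControlMode to select tiles, place towers or spawn consumables.
; Placement replaces tile actors, storing the previous tile and carrying turret upgrade state through moves.
; Tutorial events are gated by step index, advancing the widget and starting tutorial waves.
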(event Custom|Deselect
  ;[1 1 1] Tile Selection
  (Variables|Default|SetbHasSelectedTile false)
  (Utilities|ClearGradients
    (:%20%20
      (Widget|RemovefromParent (Variables|Default|GetSelection%20Widget)))))

(event Custom|Replace%20Tile
  (params (Old%20Tile :type Tile%20BP%20Object%20Reference) (New%20Tile :type Tile%20BP%20Class%20Reference))
  ;[1 1 1] Replace Tile
  (Utilities|ReplaceTile(Object) Old%20Tile New%20Tile))

(event Custom|Tutorial%20Upgrade
  ;[1 1 1] Tutorial Events
  (Utilities|CheckTutorial 4
    (:%20%20
      (CallFunction|UpdateTutorial))))

(event Custom|Tutorial%20Lumber%20Hut
  (bind _tutorial_widget (Variables|Tutorial|GetTutorial%20Widget))
  ;[1 1 1] Tutorial Events
  (Utilities|CheckTutorial 5
    (:%20%20
      (CallFunction|UpdateTutorial)
      (Utilities|FlowControl|Delay 1e+01)
      (Utilities|IsValid _tutorial_widget
        (:Is%20Valid
          (Widget|RemovefromParent _tutorial_widget))))))

(event Custom|Player%20Begin
  (bind _in_game_widget (Variables|Default|GetIn-Game%20Widget))
  ;[1 1 1] Init UI
  (Default|UpdateMoneyAmount _in_game_widget (Variables|Defaults|GetMoney))
  (Default|UpdateGoldAmount _in_game_widget (Variables|Defaults|GetGold))
  (bind _returnvalue (UserInterface|CreateWidget "/Game/BP/Widget/Selection_Widget.Selection_Widget_C" (Game|GetPlayerController 0)))
  (Variables|Default|SetSelection%20Widget _returnvalue)
  ;[1 1 1] Init Spec
  (bind _returnvalue_2 (Game|SpawnActorfromClass "/Game/BP/Cin_Pawn.Cin_Pawn_C" (Math|Transform|MakeTransform (Transformation|GetActorLocation) "0, 0, 0" "1,1,1") "Undefined" 0 0))
  (Variables|Default|SetSpectator _returnvalue_2)
  ;[1 1 1] Init Tutorial
  (bind _output_get (Variables|Tutorial|SetbTutorial (Variables|/Game/BP/Global_GI.Global_GI_C|GetbTutorial (Utilities|GameInstance))))
  (if _output_get
    (bind _returnvalue_3 (UserInterface|CreateWidget "/Game/BP/Widget/Tutorial_BP.Tutorial_BP_C" (Game|GetPlayerController 0)))
    (bind _output_get_2 (Variables|Tutorial|SetTutorial%20Widget _returnvalue_3))
    (UserInterface|Viewport|AddtoViewport _output_get_2 99)))

(event Custom|Tutorial%20Buy%20Turrets
  ;[1 1 1] Tutorial Events
  (Utilities|CheckTutorial
    (:%20%20
      (CallFunction|UpdateTutorial))))

(event Custom|Tutorial%20Place%20Turrets
  ;[1 1 1] Tutorial Events
  (Utilities|CheckTutorial 1
    (:%20%20
      (CallFunction|UpdateTutorial)
      (Default|StartWavesTutorial (Variables|Default|GetEnemy%20Spawn)))))

(event Custom|Tutorial%20Killed%20Wave
  ;[1 1 1] Tutorial Events
  (Utilities|CheckTutorial 2
    (:%20%20
      (CallFunction|UpdateTutorial))))

(event Custom|Tutorial%20Lamp%20Event
  ;[1 1 1] Tutorial Events
  (Utilities|CheckTutorial 3
    (:%20%20
      (CallFunction|UpdateTutorial))))

(event Custom|Pause
  ;[1 1 1] Pause
  (bind _returnvalue (UserInterface|CreateWidget "/Game/BP/Widget/PauseMenu_BP.PauseMenu_BP_C" (Game|GetPlayerController 0)))
  (UserInterface|Viewport|AddtoViewport _returnvalue 0))

(event EventTick
  (params (DeltaSeconds :type Float%20%28single-precision%29))
  (bind _returnvalue (Game|GetPlayerController 0))
  (bind _tower_widget (Variables|Default|GetTower%20Widget))
  (bind (_hitresult _returnvalue_2) (Game|Player|GetHitResultUnderCursorbyChannel _returnvalue "TraceTypeQuery1" true))
  ;[1 1 1] Tile Selection
  (Utilities|FlowControl|Sequence
    (:then_0
      (if _returnvalue_2
        (bind _astile_bp (Utilities|Casting|CastToTile_BP (.HitActor (Collision|BreakHitResult _hitresult))))
        (if (not (Variables|Default|GetbSpectating))
          ;[1 1 1] Hover
          (bind _outactors (Actor|GetAllActorsOfClass "/Game/BP/Tile_BP.Tile_BP_C"))
          (for _array_element _outactors
            (if (!= _array_element _astile_bp)
              (Default|DisableHoverGradient _array_element)
              (Default|StopPreviewingRadius _array_element)))
          (Default|EnableHoverGradient _astile_bp (Utilities|Select :Index (Variables|Default|GetControl%20Mode) :NewEnumerator0 "/Game/Material/Gradient/GrayGradient_BP.GrayGradient_BP" :NewEnumerator2 "/Game/Material/Gradient/GreenGradient_M.GreenGradient_M" :NewEnumerator4 "/Game/Material/Gradient/RedGradient_M.RedGradient_M"))
          (Utilities|IfMode "NewEnumerator2"
            (:True
              (bind _returnvalue_3 (Game|SpawnActorfromClass (Utilities|GetTurretClass (Variables|Default|GetCurrent%20Tower)) (Math|Transform|MakeTransform "0, 0,-10000.000000" "0, 0, 0" "1,1,1") "Undefined" 0 0))
              (Default|PreviewRadius _astile_bp (Variables|/Game/BP/Tiles/PlayerTiles/PlayerTile_BP.PlayerTile_BP_C|GetFunction%20Radius _returnvalue_3))
              (Actor|DestroyActor _returnvalue_3))))))
    (:then_1
      ;[1 1 1] Update Tower Images
      (Utilities|IsValid _tower_widget
        (:Is%20Valid
          (Default|UpdateImages _tower_widget))))
    (:then_2
      ;[1 1 1] Tutorial Placing
      (if (>= (Variables|Tutorial|GetMG%20count) 3)
        (Utilities|CheckTutorial 1
          (:%20%20
            (Utilities|FlowControl|DoOnce false
              (:Completed
                (CallFunction|TutorialPlaceTurrets)))))))))

(event Input|ActionEvents|InputActionSelectTile
  (params (Key :type Key%20Structure :default "None"))
  (bind _returnvalue (Game|GetPlayerController 0))
  (bind _selection_widget (Variables|Default|GetSelection%20Widget))
  (bind _selection_widget_2 (Variables|Default|GetSelection%20Widget))
  (bind (_hitresult _returnvalue_2) (Game|Player|GetHitResultUnderCursorbyChannel _returnvalue "TraceTypeQuery1" true))
  ;[1 1 1] Tile Selection
  (:Pressed
    (Utilities|NotinTurretMenu
      (:%20
        (if _returnvalue_2
          (bind _astile_bp (Utilities|Casting|CastToTile_BP (.HitActor (Collision|BreakHitResult _hitresult))))
          (switch Utilities|FlowControl|Switch|SwitchonControlMode (Variables|Default|GetControl%20Mode)
            (:NewEnumerator0
              ;[1 1 1] Select
              (if (not (== _astile_bp (Variables|Default|GetSelected%20Tile)))
                (Utilities|ClearGradients
                  (:%20%20
                    (Utilities|IsValid _selection_widget
                      (:Is%20Valid
                        (Widget|RemovefromParent _selection_widget))
                      (:Is%20Not%20Valid
                        _))
                    (Default|EnableGradient _astile_bp "/Game/Material/Gradient/BlueGradient_M.BlueGradient_M")
                    (Variables|Default|SetSelected%20Tile _astile_bp)
                    (UserInterface|Viewport|AddtoViewport _selection_widget_2 0)
                    (Default|UpdateSelection _selection_widget_2 _astile_bp)
                    (Variables|Default|SetbHasSelectedTile true)))))
            (:NewEnumerator2
              ;[1 1 1] Place
              (if (Variables|/Game/BP/Tile_BP.Tile_BP_C|GetbBuildable _astile_bp)
                (Utilities|ClearGradients
                  (:%20%20
                    (if (Utilities|Enum|Equal(Enum) (Variables|Default|GetControl%20Mode) "NewEnumerator2")
                      (Variables|Default|SetTile%20Material%20Pending%20Kill (Variables|/Game/BP/Tile_BP.Tile_BP_C|GetBase%20Material _astile_bp))
                      (Variables|Default|SetTile%20Pending%20Kill (Utilities|GetClass _astile_bp))
                      (bind _new_tile_ref (Utilities|ReplaceTile(Object) _astile_bp (Utilities|GetTurretClass (Variables|Default|GetCurrent%20Tower))))
                      (bind _asplayer_tile_bp (Utilities|Casting|CastToPlayerTile_BP _new_tile_ref)
                        (:then
                          (Default|SetPreviousTile _asplayer_tile_bp (Variables|Default|GetTile%20Pending%20Kill))
                          (Default|SetBaseMaterial _asplayer_tile_bp (Variables|Default|GetTile%20Material%20Pending%20Kill))
                          (bind _asturret_bp (Utilities|Casting|CastToTurret_BP _asplayer_tile_bp)
                            (:then
                              (Variables|/Game/BP/Tiles/PlayerTiles/Turret_BP.Turret_BP_C|SetCurrent%20Upgrade%20Modifier _asturret_bp (Variables|Default|GetPlaced%20Upgrade%20Modifier))
                              (Variables|/Game/BP/Tiles/PlayerTiles/Turret_BP.Turret_BP_C|SetUpgrade%20Level _asturret_bp (Variables|Default|GetPlaced%20Upgrade%20Level))
                              (Default|UpdateLVLWidget _asturret_bp))
                            (:CastFailed
                              _)))
                        (:CastFailed
                          _))
                      (Variables|Default|SetControl%20Mode "NewEnumerator0")
                      (Audio|PlaySoundatLocation "/Game/Sounds/Other/Place1-strange_dragoon.Place1-strange_dragoon" "0, 0, 0" "0, 0, 0" 1.0 1.0 0.0 0 0 0)
                      (CallFunction|SpendMoney (Variables|Default|GetCurrent%20Tower%20Spend))
                      (Utilities|FlowControl|Sequence
                        (:then_0
                          (if (Variables|Default|GetbMovingTower)
                            (Variables|Default|SetbMovingTower false)
                            (Variables|Default|SetPlaced%20Upgrade%20Level 1)
                            (Variables|Default|SetPlaced%20Upgrade%20Modifier 1.0)))
                        (:then_1
                          ;[1 1 1] Tutorial Placing
                          (Utilities|Casting|CastToMG_BP _asturret_bp)
                          (Math|Integer|IncrementInt (Variables|Tutorial|GetMG%20count)))
                        (:then_2
                          (Utilities|Casting|CastToLampRed_BP _asplayer_tile_bp)
                          (CallFunction|TutorialLampEvent))
                        (:then_3
                          (Utilities|Casting|CastToLumberHut_BP _asplayer_tile_bp)
                          (CallFunction|TutorialLumberHut))))))))
            (:NewEnumerator4
              ;[1 1 1] Consumable
              (Utilities|ClearGradients
                (:%20%20
                  (if (Utilities|Enum|Equal(Enum) (Variables|Default|GetControl%20Mode) "NewEnumerator4")
                    (if (CallFunction|CheckMoney (Variables|Default|GetCurrent%20Consumable%20Spend))
                      (Game|SpawnActorfromClass (Utilities|GetConsumableClass (Variables|Default|GetCurrent%20Consumable)) (Math|Transform|MakeTransform (Transformation|GetActorLocation _astile_bp) "0, 0, 0" "1,1,1") "Undefined" 0 0)
                      (CallFunction|SpendMoney (Variables|Default|GetCurrent%20Consumable%20Spend))
                      (else
                        (Variables|Default|SetControl%20Mode "NewEnumerator0")))))))))))))

(event Input|ActionEvents|InputActionDeselect
  (params (Key :type Key%20Structure :default "None"))
  ;[1 1 1] Tile Selection
  (:Pressed
    (Utilities|FlowControl|Sequence
      (:then_0
        (Variables|Default|SetbHasSelectedTile false)
        (Utilities|ClearGradients
          (:%20%20
            (Widget|RemovefromParent (Variables|Default|GetSelection%20Widget)))))
      (:then_1
        (if (not (Variables|Default|GetbMovingTower))
          (switch Utilities|FlowControl|Switch|SwitchonControlMode (Variables|Default|GetControl%20Mode)
            (:NewEnumerator2
              _)
            (:NewEnumerator4
              _))
          (CallFunction|SetControlMode "NewEnumerator0"))))))

(event Input|ActionEvents|InputActionAdvancetoWave99
  (params (Key :type Key%20Structure :default "None"))
  ;[1 1 1] Cheats
  (:Pressed
    (Utilities|CheatsEnabled
      (:%20
        (bind _outactors (Actor|GetAllActorsOfClass "/Game/BP/Tiles/PlayerTiles/EnemySpawn_BP.EnemySpawn_BP_C"))
        (for _array_element _outactors
          (Variables|/Game/BP/Tiles/PlayerTiles/EnemySpawn_BP.EnemySpawn_BP_C|SetCurrent%20Wave _array_element 99)
          (Default|UpdateGamemodeWave _array_element))))))

(event Input|ActionEvents|InputActionPan
  (params (Key :type Key%20Structure :default "None"))
  ;[1 1 1] Panning
  (:Pressed
    (Utilities|GameMode)
    (Variables|Default|SetbPanning true))
  (:Released
    (Utilities|UIMode (Variables|Default|GetIn-Game%20Widget))
    (Variables|Default|SetbPanning false)))

(event Input|ActionEvents|InputActionPause
  (params (Key :type Key%20Structure :default "None"))
  ;[1 1 1] Pause
  (:Pressed
    (bind _returnvalue (UserInterface|CreateWidget "/Game/BP/Widget/PauseMenu_BP.PauseMenu_BP_C" (Game|GetPlayerController 0)))
    (UserInterface|Viewport|AddtoViewport _returnvalue 0)))

(event Input|ActionEvents|InputActionCinematicCamera
  (params (Key :type Key%20Structure :default "None"))
  ;[1 1 1] Cin Camera
)

(event Input|ActionEvents|InputActionExitMenu
  (params (Key :type Key%20Structure :default "None"))
  (bind _tower_widget (Variables|Default|GetTower%20Widget))
  ;[1 1 1] Exit Menu
  (:Pressed
    (Utilities|IsValid _tower_widget
      (:Is%20Valid
        (Default|ExitMenu _tower_widget)))))

(event Input|ActionEvents|InputActionTurretMenu
  (params (Key :type Key%20Structure :default "None"))
  ;[1 1 1] Exit Menu
  (:Pressed
    (bind ___ (Utilities|NotinTurretMenu)
      (:%20
        (Default|Buy ___)))))

(event Input|ActionEvents|InputActionAdditionalMoney
  (params (Key :type Key%20Structure :default "None"))
  ;[1 1 1] Cheats
  (:Pressed
    (Utilities|CheatsEnabled
      (:%20
        (CallFunction|GainMoney 2000)))))

(event Input|ActionEvents|InputActionAdditionalGold
  (params (Key :type Key%20Structure :default "None"))
  ;[1 1 1] Cheats
  (:Pressed
    (Utilities|CheatsEnabled
      (:%20
        (CallFunction|GainGold 2000)))))

(event Input|AxisEvents|InputAxisMouseX
  (params (AxisValue :type Float%20%28single-precision%29))
  ;[1 1 1] Panning
  (if (Variables|Default|GetbPanning)
    (Transformation|AddLocalOffset (Variables|Default|GetCamera) (* (Transformation|GetActorRightVector) (* (Utilities|Invert(float) AxisValue) (Variables|Visual|GetDrag%20Speed))) false false)))

(event Input|AxisEvents|InputAxisMouseY
  (params (AxisValue :type Float%20%28single-precision%29))
  ;[1 1 1] Panning
  (if (Variables|Default|GetbPanning)
    (Transformation|AddActorLocalOffset (* (Math|Vector|Normalize (+ (Transformation|GetActorForwardVector) (Transformation|GetActorRightVector))) (* (Utilities|Invert(float) AxisValue) (Variables|Visual|GetDrag%20Speed))) false false)))

(event Input|AxisEvents|InputAxisZoom
  (params (AxisValue :type Float%20%28single-precision%29))
  (bind _zoom_limits (Variables|Default|GetZoom%20Limits))
  (bind _zoom_speed (Variables|Visual|GetZoom%20Speed))
  (bind _returnvalue (* AxisValue _zoom_speed))
  ;[1 1 1] Panning
  (bind _output_get (Variables|Default|SetbPositiveZoom (> _returnvalue 0.0)))
  (bind _output_get_2 (Variables|Default|SetbNegativeZoom (< _returnvalue 0.0)))
  (if _output_get ; Positive Zoom
    (if (< (Variables|Default|GetZoom%20Amount) (.x _zoom_limits))
      (Transformation|AddLocalOffset (Variables|Default|GetCamera) (* (Transformation|GetActorForwardVector) _returnvalue) false false :!label _label)
      (Variables|Default|SetZoom%20Amount (+ (Variables|Default|GetZoom%20Amount) _returnvalue)))
    (elif _output_get_2 ; Negative Zoom
      (if (> (Variables|Default|GetZoom%20Amount) (.y _zoom_limits))
        (goto _label)))))

(fn ConstructionScript)

(fn CheckMoney
  (params (Amount :type Integer))
  (return (<= Amount (Variables|Defaults|GetMoney))))

(fn SpendMoney
  (params (Amount :type Integer))
  (bind _output_get (Variables|Defaults|SetMoney (- (Variables|Defaults|GetMoney) Amount)))
  (Default|UpdateMoneyAmount (Variables|Default|GetIn-Game%20Widget) _output_get))

(fn PlaceTower
  (params (Tower :type Turret_Enum%20Enum :default "NewEnumerator0") (Placed%20Upgrade%20Modifier :type Float%20%28single-precision%29) (Spend :type Integer) (Placed%20Upgrade%20Level :type Integer))
  (Variables|Default|SetPlaced%20Upgrade%20Modifier Placed%20Upgrade%20Modifier)
  (Variables|Default|SetPlaced%20Upgrade%20Level Placed%20Upgrade%20Level)
  (Variables|Default|SetCurrent%20Tower%20Spend Spend)
  (Variables|Default|SetControl%20Mode "NewEnumerator2")
  (Variables|Default|SetCurrent%20Tower Tower))

(fn GainMoney
  (params (Amount :type Integer))
  (bind _output_get (Variables|Defaults|SetMoney (+ Amount (Variables|Defaults|GetMoney))))
  (Default|UpdateMoneyAmount (Variables|Default|GetIn-Game%20Widget) _output_get))

(fn CheckGold
  (params (Amount :type Integer))
  (return (<= Amount (Variables|Defaults|GetGold))))

(fn SpendGold
  (params (Amount :type Integer))
  (bind _output_get (Variables|Defaults|SetGold (- (Variables|Defaults|GetGold) Amount)))
  (Default|UpdateGoldAmount (Variables|Default|GetIn-Game%20Widget) _output_get))

(fn GainGold
  (params (Amount :type Integer))
  (bind _output_get (Variables|Defaults|SetGold (+ Amount (Variables|Defaults|GetGold))))
  (Default|UpdateGoldAmount (Variables|Default|GetIn-Game%20Widget) _output_get))

(fn SetControlMode
  (params (Control%20Mode :type ControlMode%20Enum :default "NewEnumerator0"))
  (Variables|Default|SetControl%20Mode Control%20Mode))

(fn UpdateTutorial
  (bind _result (Math|Integer|IncrementInt (Variables|Tutorial|GetTutorial%20Index))
    (:%20%20
      (Default|Update (Variables|Tutorial|GetTutorial%20Widget) _result))))

(fn UseConsumable
  (params (Consumable :type Consumable%20Enum :default "NewEnumerator0") (Price :type Integer))
  (Variables|Default|SetCurrent%20Consumable Consumable)
  (Variables|Default|SetCurrent%20Consumable%20Spend Price)
  (CallFunction|SetControlMode "NewEnumerator4"))