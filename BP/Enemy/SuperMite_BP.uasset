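; SuperMite_BP is a child enemy Blueprint for a waypoint-following wave enemy that splits into smaller mites when killed.
; It loads its stats from the SuperMite row of the enemy properties data table.
; On Kill it runs the parent logic, then spawns MiteCount Mite_BP actors at nearby random navigable points.
; Each mite is advanced to the parent's waypoint index and added to the GameInstance's wave enemy list.
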(event EventBeginPlay
  (|CallParentFunction) ; This node is disabled and will not be called.\nDrag off pins to build functionality.
)

(event Collision|EventActorBeginOverlap
  (params (OtherActor :type Actor%20Object%20Reference)))

(event EventTick
  (params (DeltaSeconds :type Float%20%28single-precision%29))
  (|CallParentFunction DeltaSeconds) ; This node is disabled and will not be called.\nDrag off pins to build functionality.
)

(event EventKill
  (|CallParentFunction)
  (for _index (range 1 (Variables|Default|GetMite%20Count))
    (bind _returnvalue (Game|SpawnActorfromClass "/Game/BP/Enemy/Mite_BP.Mite_BP_C" (Math|Transform|MakeTransform (.RandomLocation (Class|NavigationSystemV1|GetRandomPointinNavigableRadius (Transformation|GetActorLocation) 1e+02 0 0)) "0, 0, 0" "1,1,1") "AdjustIfPossibleButAlwaysSpawn" 0 0))
    (for _index_2 (range 1 (Variables|Default|GetCurrent%20Waypoint%20Index))
      (Default|UpdateWaypoint _returnvalue))
    (Utilities|Array|Add (Variables|/Game/BP/Tiles/PlayerTiles/EnemySpawn_BP.EnemySpawn_BP_C|GetWave%20Enemies (Variables|/Game/BP/Global_GI.Global_GI_C|Getspawn (Utilities|GameInstance))) _returnvalue)))

(event EventInitDataTable
  (bind _returnvalue (Utilities|GetDataTableRow "/Game/BP/Enemy/EnemyProperties_table.EnemyProperties_table" "SuperMite")
    (:then
      (Variables|Default|SetProperties _returnvalue))))

(fn ConstructionScript
  (|CallParentFunction))