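; Enemy pawn that follows indexed waypoints, takes damage, poison and stuns, and can damage a base, with stats from a data table.
; Waypoint updates restart AI MoveTo, while damage drives a dynamic-material health bar.
; Death ragdolls the mesh with knockback, pays the player, then hides it after a timeout.
; Tick flags it as lit near lamps or auto-lighting actors and kills it below Kill Z or when stuck.
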(event Custom|Stun
  (params (Time :type Float%20%28single-precision%29))
  (bind _charactermovement (Variables|Character|GetCharacterMovement))
  ;[1 1 1] Stun
  (if (> Time 0.0)
    (if (not (Variables|Default|GetbStunned))
      (Variables|Default|SetLatest%20Stun%20Time Time)
      (Variables|Default|SetbStunned true)
      (Variables|/Script/Engine.CharacterMovementComponent|SetMaxWalkSpeed _charactermovement 0.0)
      (Utilities|FlowControl|Delay (Variables|Default|GetLatest%20Stun%20Time))
      (Variables|/Script/Engine.CharacterMovementComponent|SetMaxWalkSpeed _charactermovement (Variables|Default|GetInitial%20Walk%20Speed))
      (Variables|Default|SetbStunned false))))

(event Custom|Update%20Waypoint
  ;[1 1 1] Waypoints
  (Math|Integer|IncrementInt (Variables|Default|GetCurrent%20Waypoint%20Index)
    (:%20%20
      (bind __ (CallFunction|GetCurrentWaypoint))
      (AI|AIMoveTo self "0, 0, 0" __ 5.0 false))))

(event Custom|Poison
  (params (Poison :type Float%20%28single-precision%29) (Duration :type Integer) (Effect :type Particle%20System%20Object%20Reference))
  ;[1 1 1] Poison
  (if (> Poison 0.01)
    (if (not (Variables|Default|GetbDead))
      (if (not (Variables|Default|GetbPoisoned))
        (Variables|Default|SetLatest%20Poison%20Amount Poison)
        (Variables|Default|SetLatest%20Poison%20Duration Duration)
        (Variables|Default|SetbPoisoned true)
        (bind _returnvalue (Effects|SpawnEmitterAttached Effect (Variables|Character|GetMesh) "Base" "0, 0, 0" "0, 0, 0" "0.100000,0.100000,0.100000" "KeepRelativeOffset" false))
        (Variables|Default|SetPoison%20Effect _returnvalue)
        (Utilities|ForLoopwithDelay 1 (Variables|Default|GetLatest%20Poison%20Duration) (Variables|Default|GetPoison%20Delay)
          (:Loop%20Body
            (CallFunction|Damage (Variables|Default|GetLatest%20Poison%20Amount)))
          (:Completed
            (Components|DestroyComponent (Variables|Default|GetPoison%20Effect))
            (Variables|Default|SetbPoisoned false)))))))

(event EventBeginPlay
  (bind _properties (Variables|Default|GetProperties))
  (Utilities|FlowControl|Sequence
    (:then_0
      ;[1 1 1] Init Health Bar
      (bind _returnvalue (Rendering|Material|CreateDynamicMaterialInstance (Variables|Properties|GetHeatBar_MI) "None" :!class /Script/Engine.KismetMaterialLibrary))
      (bind _output_get (Variables|Default|SetHealth%20Bar%20Instance _returnvalue))
      (Rendering|Material|SetMaterial (Variables|Default|GetHealth%20Bar) 0 _output_get)
      ;[1 1 1] Init Data Table
      (CallFunction|InitDataTable)
      ;[1 1 1] Init
      (Variables|Default|SetCurrent%20Health (.health _properties))
      (bind _output_get_2 (Variables|/Script/Engine.CharacterMovementComponent|SetMaxWalkSpeed (Variables|Character|GetCharacterMovement) (.speed _properties)))
      (Variables|Default|SetInitial%20Walk%20Speed _output_get_2)
      ;[1 1 1] Waypoints
      (bind __ (CallFunction|GetCurrentWaypoint))
      (Transformation|SetActorRotation (Math|Rotator|FindLookatRotation (Transformation|GetActorLocation) (Transformation|GetActorLocation __)))
      (Utilities|FlowControl|Delay 0.1)
      (bind ___2 (CallFunction|GetCurrentWaypoint))
      (AI|AIMoveTo self "0, 0, 0" ___2 5.0 false))
    (:then_1
      ;[1 1 1] Entry Emitter
      (Effects|SpawnEmitteratLocation "/Game/Particle/TealEntrance_BP.TealEntrance_BP" (Transformation|GetActorLocation)))))

(event EventTick
  (params (DeltaSeconds :type Float%20%28single-precision%29))
  (Utilities|FlowControl|Sequence
    (:then_0
      ;[1 1 1] Death Timeout
      (if (Variables|Default|GetbDead)
        (Utilities|FlowControl|DoOnce false
          (:Completed
            (Components|DestroyComponent (Variables|Default|GetPoison%20Effect))
            (Utilities|FlowControl|Delay (Variables|Default|GetDeath%20Timeout))
            (CallFunction|DeathTimeoutEvents)))))
    (:then_1
      ;[1 1 1] Lighting
      (Utilities|Array|Clear (Variables|Default|GetLamps))
      (Variables|Default|SetbLit false)
      (bind _outactors (Actor|GetAllActorsOfClass "/Game/BP/Tiles/PlayerTiles/Lamp_BP.Lamp_BP_C"))
      (bind _output_get (Variables|Default|SetLamps _outactors))
      (bind _outactors_2 (Actor|GetAllActorsOfClass "/Game/BP/Tiles/PlayerTiles/LampRed_BP.LampRed_BP_C"))
      (Utilities|Array|AppendArray _output_get _outactors_2)
      (for _array_element _output_get
        (if (not (Variables|Default|GetbLit))
          (if (< (Transformation|GetDistanceTo _array_element) (Variables|/Game/BP/Tiles/PlayerTiles/PlayerTile_BP.PlayerTile_BP_C|GetFunction%20Radius _array_element))
            (Variables|Default|SetbLit true))))
      ;[1 1 1] Auto Lighting
      (for _array_element_2 (Variables|Default|GetAuto%20Lighting%20Actors)
        (bind _outactors_3 (Actor|GetAllActorsOfClass _array_element_2))
        (for _array_element_3 _outactors_3
          (if (not (Variables|Default|GetbLit))
            (if (< (Transformation|GetDistanceTo _array_element_3) (Variables|Default|GetAuto%20Lighting%20Radius))
              (Variables|Default|SetbLit true))))))
    (:then_2
      ;[1 1 1] Kill Z
      (if (< (.z (Transformation|GetActorLocation)) (Variables|Default|GetKillz))
        (if (not (Variables|Default|GetbDead))
          (CallFunction|Damage 999999995904.0))))
    (:then_3
      ;[1 1 1] Bug Fix
      (Variables|Default|SetBug%20Timer (+ (Variables|Default|GetBug%20Timer) (Utilities|Time|GetWorldDeltaSeconds)))
      (Utilities|FlowControl|Sequence
        (:then_0
          (if (> (Math|Vector|VectorLength (Transformation|GetVelocity)) 0.001)
            (Variables|Default|SetBug%20Timer 0.0)))
        (:then_1
          (if (>= (Variables|Default|GetBug%20Timer) 5.0)
            (if (not (Variables|Default|GetbDead))
              (CallFunction|Kill))))))))

(fn ConstructionScript)

(fn UpdateWaypoints)

(fn CheckWaypoint
  (params (%20 :type Integer))
  (return (== %20 (Variables|Default|GetCurrent%20Waypoint%20Index))))

(fn GetCurrentWaypoint
  (for _array_element (Variables|/Game/BP/MainGamemode_BP.MainGamemode_BP_C|GetWaypoints (Utilities|Gamemode))
    (if (CallFunction|CheckWaypoint (Variables|/Game/BP/WayPoint_BP.WayPoint_BP_C|GetIndex _array_element))
      (LocalVariables|SetWaypoint _array_element)))
  (return (LocalVariables|GetWaypoint)))

(fn InitDataTable
  (bind _returnvalue (Utilities|GetDataTableRow "/Game/BP/Enemy/EnemyProperties_table.EnemyProperties_table" "Enemy")
    (:then
      (Variables|Default|SetProperties _returnvalue))))

(fn Damage
  (params (Amount :type Float%20%28single-precision%29))
  (if (not (Variables|Default|GetbDead))
    (Variables|Default|SetCurrent%20Health (- (Variables|Default|GetCurrent%20Health) Amount))
    (CallFunction|UpdateHealthBar)
    (if (<= (Variables|Default|GetCurrent%20Health) 0.0)
      (CallFunction|Kill))))

(fn Kill
  (bind _mesh (Variables|Character|GetMesh))
  (Collision|SetCollisionEnabled _mesh "PhysicsOnly")
  (Physics|SetSimulatePhysics _mesh true)
  (Collision|SetCollisionEnabled (Variables|Collision|GetCapsuleComponent) "NoCollision")
  (Physics|AddImpulse (Variables|Character|GetMesh) (Variables|Default|GetKO) "Base" false)
  (Default|GainMoney (Utilities|Player) (.moneygain (Variables|Default|GetProperties)))
  (Variables|Default|SetbDead true)
  (CallFunction|SetHealthBarVisibility false)
  (Class|Pawn|DetachfromControllerPendingDestroy))

(fn SetKnockback
  (params (Amount :type Float%20%28single-precision%29) (Direction :type Rotator))
  (Variables|Default|SetKO (Math|Vector|RotateVector (Math|Vector|MakeVector Amount 0.0 0.0) Direction)))

(fn Destroy
  (Actor|DestroyActor))

(fn UpdateHealthBar
  (Rendering|Material|SetScalarParameterValue (Variables|Default|GetHealth%20Bar%20Instance) "Progress" (/ (Variables|Default|GetCurrent%20Health) (* (.health (Variables|Default|GetProperties)) (Variables|Default|GetHealth%20Modifier))) :!class /Script/Engine.MaterialInstanceDynamic))

(fn SetHealthBarVisibility
  (params (Visible :type Boolean))
  (Rendering|SetVisibility (Variables|Default|GetHealth%20Bar) Visible false)
  (return))

(fn SetHealthModifier
  (params (Health%20Modifier :type Float%20%28single-precision%29))
  (Variables|Default|SetHealth%20Modifier Health%20Modifier)
  (Variables|Default|SetCurrent%20Health (* (Variables|Default|GetCurrent%20Health) (Variables|Default|GetHealth%20Modifier))))

(fn DamageBase
  (params (Base :type Player%20Base%20BP%20Object%20Reference))
  (Variables|Default|SetKO "0, 0,20000.000000")
  (Effects|SpawnEmitteratLocation "/Game/Particle/FireLarge_Exp_P.FireLarge_Exp_P" (Transformation|GetActorLocation))
  (CallFunction|Kill)
  (Default|Damage Base (.basedamage (Variables|Default|GetProperties))))

(fn DeathTimeoutEvents
  (Effects|SpawnEmitteratLocation "/Game/Particle/Teal_Exp_P.Teal_Exp_P" (Transformation|GetSocketLocation (Variables|Character|GetMesh) "Base"))
  (Rendering|SetVisibility (Variables|Character|GetMesh) false false)
  (Rendering|Components|Light|SetIntensity (Variables|Default|GetSpotLight) 0.0))