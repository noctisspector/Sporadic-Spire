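; Slug enemy Blueprint, a child enemy class that stuns nearby turrets when killed.
; It loads its stats from the "Slug" row of the enemy properties data table.
; On kill it runs the parent logic, spawns a stun particle effect and calls Stun on every Turret_BP actor within StunRange.
; The death timeout event also runs the parent logic, then sets both spotlights to zero intensity.
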(event EventBeginPlay
  (|CallParentFunction) ; This node is disabled and will not be called.\nDrag off pins to build functionality.
)

(event Collision|EventActorBeginOverlap
  (params (OtherActor :type Actor%20Object%20Reference)))

(event EventTick
  (params (DeltaSeconds :type Float%20%28single-precision%29))
  (|CallParentFunction DeltaSeconds) ; This node is disabled and will not be called.\nDrag off pins to build functionality.
)

(event EventInitDataTable
  (bind _returnvalue (Utilities|GetDataTableRow "/Game/BP/Enemy/EnemyProperties_table.EnemyProperties_table" "Slug")
    (:then
      (Variables|Default|SetProperties _returnvalue))))

(event EventDeathTimeoutEvents
  (|CallParentFunction)
  (Rendering|Components|Light|SetIntensity (Variables|Default|GetSpotLight1) 0.0)
  (Rendering|Components|Light|SetIntensity (Variables|Default|GetSpotLight2) 0.0))

(event EventKill
  (|CallParentFunction)
  (Effects|SpawnEmitteratLocation "/Game/Particle/SlugStun_P.SlugStun_P" (Transformation|GetActorLocation))
  (bind _outactors (Actor|GetAllActorsOfClass "/Game/BP/Tiles/PlayerTiles/Turret_BP.Turret_BP_C"))
  (for _array_element _outactors
    (if (< (Transformation|GetDistanceTo _array_element) (Variables|Default|GetStun%20Range))
      (Default|Stun _array_element (Variables|Default|GetStun%20Time)))))

(fn ConstructionScript
  (|CallParentFunction))